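; Tank spell for grid-based tactics that shoves the unit next to the caster away along a line, spending caster initiative.
; Targeting highlights forward-filtered tiles, with extra range from height 2.
; PushFunctionLv2 pushes one tile or steps toward the clicked tile, resolving collision and height-drop damage.
; ReduceInit sets cost by Manhattan distance; the older PushActionResult/PushObjectResult path is disconnected.
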(event EventEShowTilesTargetedbySpell
  (params (Origin%20Index :type Vector%202D%20Structure) (Grid :type Grid%20Behaviours%20Object%20Reference) (Show%20Tiles :type Boolean))
  (if (== (Variables|/Game/01_BP/03_Character/TopDownCharacter.TopDownCharacter_C|GetPlayerHeight (Variables|Default|GetSpellOwner)) 2)
    (Math|Integer|IncrementInt (Variables|Default|GetcurrentDistance)
      (:%20%20
        _)))
  (if (> (Utilities|Array|Length (Variables|Default|GetReachableTarget)) 0)
    (Default|HighlightAttackableTiles Grid (Variables|Default|GetReachableTarget) false)
    (Utilities|Array|Clear (Variables|Default|GetAttackableTiles))
    (Utilities|Array|Clear (Variables|Default|GetUnAttackableTiles))
    (Utilities|Array|Clear (Variables|Default|GetReachableTarget)))
  (bind _newlocalvar_01 (CallFunction|GetAttackableTiles Origin%20Index Grid))
  (bind _reachablestargets (CallFunction|GetReachableTargetatMinimumDistances _newlocalvar_01 Origin%20Index))
  (bind _reachabletiles (CallFunction|CheckForward _reachablestargets))
  (bind _output_get (Variables|Default|SetReachableTarget _reachabletiles))
  (Default|HighlightAttackableTiles Grid _output_get Show%20Tiles))

(event EventBeginPlay
  (|CallParentFunction)
  (Variables|Value|SetTempCost (Variables|Default|Getm_Cost)))

(event EventEUseSpellonTarget
  (params (Grid :type Grid%20Behaviours%20Object%20Reference) (Target%20position :type Vector%202D%20Structure) (SpellOwner :type Top%20Down%20Character%20Object%20Reference))
  (bind (_x _y) (Math|Vector2D|BreakVector2D Target%20position))
  (if (and (> _x 0.0) (> _y 0.0))
    (CallFunction|PushFunctionLv2 Grid Target%20position)
    (CallFunction|ReduceInit Target%20position)
    (Variables|Default|Setm_Cost (Variables|Value|GetTempCost))
    (Variables|Default|SetcurrentDistance (Variables|Default|Getm_Distances))
    (Default|EDeselectSpeel SpellOwner)
    (else
      (Class|FMODAudioComponent|Play (Variables|Default|GetCantAttaque_FMODAudio)))))

(fn ConstructionScript
  (|CallParentFunction))

(fn PushActionResult
  (params (SpeelTarget :type Top%20Down%20Character%20Object%20Reference) (SpeelCaster :type Top%20Down%20Character%20Object%20Reference) (GridManager :type Grid%20Behaviours%20Object%20Reference))
  (LocalVariables|SetTarget SpeelTarget)
  (LocalVariables|SetCaster SpeelCaster)
  (LocalVariables|SetGrid GridManager)
  (if (> (Variables|/Game/01_BP/03_Character/TopDownCharacter.TopDownCharacter_C|GetPlayerHeight (LocalVariables|GetTarget)) (Variables|/Game/01_BP/03_Character/TopDownCharacter.TopDownCharacter_C|GetPlayerHeight (LocalVariables|GetCaster)))
    (if (== (.unitonthistile (.Value (Utilities|Map|Find (Variables|/Game/01_BP/Grid/GridBehaviours.GridBehaviours_C|Getstruct_Tiles (LocalVariables|GetGrid)) (CallFunction|GetDirection (Variables|/Game/01_BP/03_Character/TopDownCharacter.TopDownCharacter_C|Getgrid%20Index (LocalVariables|GetTarget)) (Variables|/Game/01_BP/03_Character/TopDownCharacter.TopDownCharacter_C|Getgrid%20Index (LocalVariables|GetCaster)))))) 0)
      (if (>= (- (Variables|/Game/01_BP/03_Character/TopDownCharacter.TopDownCharacter_C|GetPlayerHeight (LocalVariables|GetTarget)) (.height (.Value (Utilities|Map|Find (Variables|/Game/01_BP/Grid/GridBehaviours.GridBehaviours_C|Getstruct_Tiles (LocalVariables|GetGrid)) (CallFunction|GetDirection (Variables|/Game/01_BP/03_Character/TopDownCharacter.TopDownCharacter_C|Getgrid%20Index (LocalVariables|GetTarget)) (Variables|/Game/01_BP/03_Character/TopDownCharacter.TopDownCharacter_C|Getgrid%20Index (LocalVariables|GetCaster))))))) 0)
        (switch int (- (Variables|/Game/01_BP/03_Character/TopDownCharacter.TopDownCharacter_C|GetPlayerHeight (LocalVariables|GetTarget)) (.height (.Value (Utilities|Map|Find (Variables|/Game/01_BP/Grid/GridBehaviours.GridBehaviours_C|Getstruct_Tiles (LocalVariables|GetGrid)) (CallFunction|GetDirection (Variables|/Game/01_BP/03_Character/TopDownCharacter.TopDownCharacter_C|Getgrid%20Index (LocalVariables|GetTarget)) (Variables|/Game/01_BP/03_Character/TopDownCharacter.TopDownCharacter_C|Getgrid%20Index (LocalVariables|GetCaster)))))))
          (:0
            _)
          (:1
            (Default|ETakeDamage (LocalVariables|GetTarget) (/ (Variables|Default|GetmaxDegats) 2)))
          (:2
            (Default|ETakeDamage (LocalVariables|GetTarget) (Variables|Default|GetmaxDegats))))
        (Transformation|SetActorLocation (LocalVariables|GetTarget) (.m_tiles_worldlocation (.Value (Utilities|Map|Find (Variables|/Game/01_BP/Grid/GridBehaviours.GridBehaviours_C|Getstruct_Tiles (LocalVariables|GetGrid)) (CallFunction|GetDirection (Variables|/Game/01_BP/03_Character/TopDownCharacter.TopDownCharacter_C|Getgrid%20Index (LocalVariables|GetTarget)) (Variables|/Game/01_BP/03_Character/TopDownCharacter.TopDownCharacter_C|Getgrid%20Index (LocalVariables|GetCaster)))))) false false)
        (Default|GetUnitonTile (LocalVariables|GetTarget) (.m_tiles_index (.Value (Utilities|Map|Find (Variables|/Game/01_BP/Grid/GridBehaviours.GridBehaviours_C|Getstruct_Tiles (LocalVariables|GetGrid)) (CallFunction|GetDirection (Variables|/Game/01_BP/03_Character/TopDownCharacter.TopDownCharacter_C|Getgrid%20Index (LocalVariables|GetTarget)) (Variables|/Game/01_BP/03_Character/TopDownCharacter.TopDownCharacter_C|Getgrid%20Index (LocalVariables|GetCaster)))))))
        (CallFunction|AffectDamage (LocalVariables|GetTarget) (.height (.Value (Utilities|Map|Find (Variables|/Game/01_BP/Grid/GridBehaviours.GridBehaviours_C|Getstruct_Tiles (LocalVariables|GetGrid)) (CallFunction|GetDirection (Variables|/Game/01_BP/03_Character/TopDownCharacter.TopDownCharacter_C|Getgrid%20Index (LocalVariables|GetTarget)) (Variables|/Game/01_BP/03_Character/TopDownCharacter.TopDownCharacter_C|Getgrid%20Index (LocalVariables|GetCaster)))))))
        (else
          (Default|ETakeDamage (LocalVariables|GetTarget) (/ (Variables|Default|GetmaxDegats) 2))))
      (elif (.bSuccess (Utilities|Casting|CastToTopDownCharacter (.unitonthistile (.Value (Utilities|Map|Find (Variables|/Game/01_BP/Grid/GridBehaviours.GridBehaviours_C|Getstruct_Tiles (LocalVariables|GetGrid)) (CallFunction|GetDirection (Variables|/Game/01_BP/03_Character/TopDownCharacter.TopDownCharacter_C|Getgrid%20Index (LocalVariables|GetTarget)) (Variables|/Game/01_BP/03_Character/TopDownCharacter.TopDownCharacter_C|Getgrid%20Index (LocalVariables|GetCaster))))))))
        (Default|ETakeDamage (.AsTop%20Down%20Character (Utilities|Casting|CastToTopDownCharacter (.unitonthistile (.Value (Utilities|Map|Find (Variables|/Game/01_BP/Grid/GridBehaviours.GridBehaviours_C|Getstruct_Tiles (LocalVariables|GetGrid)) (CallFunction|GetDirection (Variables|/Game/01_BP/03_Character/TopDownCharacter.TopDownCharacter_C|Getgrid%20Index (LocalVariables|GetTarget)) (Variables|/Game/01_BP/03_Character/TopDownCharacter.TopDownCharacter_C|Getgrid%20Index (LocalVariables|GetCaster)))))))) (/ (Variables|Default|GetmaxDegats) 2))
        (else
          ;[1 1 1] Apply a debuf on the speed
          (if (.bSuccess (Utilities|Casting|CastToBP_Base_Obstacle (.unitonthistile (.Value (Utilities|Map|Find (Variables|/Game/01_BP/Grid/GridBehaviours.GridBehaviours_C|Getstruct_Tiles (LocalVariables|GetGrid)) (CallFunction|GetDirection (Variables|/Game/01_BP/03_Character/TopDownCharacter.TopDownCharacter_C|Getgrid%20Index (LocalVariables|GetTarget)) (Variables|/Game/01_BP/03_Character/TopDownCharacter.TopDownCharacter_C|Getgrid%20Index (LocalVariables|GetCaster))))))))
            (Default|EApplyDebuff (LocalVariables|GetTarget) (Variables|Default|GetInitDebuffValue) (Variables|Default|GetDebuffTime))))))))

(fn PushObjectResult
  (params (GridManager :type Grid%20Behaviours%20Object%20Reference) (Obstacle :type BP%20Movable%20Obstacle%20Object%20Reference))
  (LocalVariables|SetGrid GridManager)
  (bind _output_get (LocalVariables|SetObstacleToPush Obstacle))
  (if (== (.unitonthistile (.Value (Utilities|Map|Find (Variables|/Game/01_BP/Grid/GridBehaviours.GridBehaviours_C|Getstruct_Tiles (LocalVariables|GetGrid)) (CallFunction|GetDirection (Variables|/Game/01_BP/07_Obstacles/BP_Base_Obstacle.BP_Base_Obstacle_C|GetGrid%20Index _output_get) (Variables|/Game/01_BP/03_Character/TopDownCharacter.TopDownCharacter_C|Getgrid%20Index (Variables|Default|GetSpellOwner)))))) 0)
    (Transformation|SetActorLocation (LocalVariables|GetObstacleToPush) (.m_tiles_worldlocation (.Value (Utilities|Map|Find (Variables|/Game/01_BP/Grid/GridBehaviours.GridBehaviours_C|Getstruct_Tiles (LocalVariables|GetGrid)) (CallFunction|GetDirection (Variables|/Game/01_BP/07_Obstacles/BP_Base_Obstacle.BP_Base_Obstacle_C|GetGrid%20Index _output_get) (Variables|/Game/01_BP/03_Character/TopDownCharacter.TopDownCharacter_C|Getgrid%20Index (Variables|Default|GetSpellOwner)))))) false false)
    (Default|SetUnitonTile (LocalVariables|GetObstacleToPush) (.m_tiles_index (.Value (Utilities|Map|Find (Variables|/Game/01_BP/Grid/GridBehaviours.GridBehaviours_C|Getstruct_Tiles (LocalVariables|GetGrid)) (CallFunction|GetDirection (Variables|/Game/01_BP/07_Obstacles/BP_Base_Obstacle.BP_Base_Obstacle_C|GetGrid%20Index _output_get) (Variables|/Game/01_BP/03_Character/TopDownCharacter.TopDownCharacter_C|Getgrid%20Index (Variables|Default|GetSpellOwner)))))))
    (elif (.bSuccess (Utilities|Casting|CastToTopDownCharacter (.unitonthistile (.Value (Utilities|Map|Find (Variables|/Game/01_BP/Grid/GridBehaviours.GridBehaviours_C|Getstruct_Tiles (LocalVariables|GetGrid)) (CallFunction|GetDirection (Variables|/Game/01_BP/07_Obstacles/BP_Base_Obstacle.BP_Base_Obstacle_C|GetGrid%20Index _output_get) (Variables|/Game/01_BP/03_Character/TopDownCharacter.TopDownCharacter_C|Getgrid%20Index (Variables|Default|GetSpellOwner))))))))
      (Default|ETakeDamage (.AsTop%20Down%20Character (Utilities|Casting|CastToTopDownCharacter (.unitonthistile (.Value (Utilities|Map|Find (Variables|/Game/01_BP/Grid/GridBehaviours.GridBehaviours_C|Getstruct_Tiles (LocalVariables|GetGrid)) (CallFunction|GetDirection (Variables|/Game/01_BP/07_Obstacles/BP_Base_Obstacle.BP_Base_Obstacle_C|GetGrid%20Index _output_get) (Variables|/Game/01_BP/03_Character/TopDownCharacter.TopDownCharacter_C|Getgrid%20Index (Variables|Default|GetSpellOwner)))))))) (/ (Variables|Default|GetmaxDegats) 2)))))

(fn PushFunctionLv2
  (params (Grid :type Grid%20Behaviours%20Object%20Reference) (Target :type Vector%202D%20Structure))
  (LocalVariables|SetGridManager Grid)
  (LocalVariables|SetClickedPosition Target)
  (LocalVariables|SetDirection (Math|Vector2D|Normalize2D (- (Variables|/Game/01_BP/03_Character/TopDownCharacter.TopDownCharacter_C|Getgrid%20Index (Variables|Default|GetSpellOwner)) (LocalVariables|GetClickedPosition))))
  (LocalVariables|SetTargetPlayer (Variables|/Game/01_BP/03_Character/TopDownCharacter.TopDownCharacter_C|Getgrid%20Index (Variables|Default|GetSpellOwner)))
  (bind _astop_down_character (Utilities|Casting|CastToTopDownCharacter (.unitonthistile (.Value (Utilities|Map|Find (Variables|/Game/01_BP/Grid/GridBehaviours.GridBehaviours_C|Getstruct_Tiles (LocalVariables|GetGridManager)) (- (LocalVariables|GetTargetPlayer) (LocalVariables|GetDirection)))))))
  (LocalVariables|SetSpellTarget _astop_down_character)
  (bind _astop_down_character_2 (Utilities|Casting|CastToTopDownCharacter (.unitonthistile (.Value (Utilities|Map|Find (Variables|/Game/01_BP/Grid/GridBehaviours.GridBehaviours_C|Getstruct_Tiles (LocalVariables|GetGridManager)) (LocalVariables|GetClickedPosition)))))
    (:then
      (if (!= _astop_down_character_2 (LocalVariables|GetSpellTarget))
        (if (Utilities|Array|ContainsItem (Variables|Default|GetReachableTarget) (LocalVariables|GetClickedPosition)) :!label _label
          (LocalVariables|Setdamage (CallFunction|GetDamage))
          (bind _index (Utilities|FlowControl|ForLoopwithBreak 0 (Math|Float|Round (CallFunction|ManhattanDistance (Variables|/Game/01_BP/03_Character/TopDownCharacter.TopDownCharacter_C|Getgrid%20Index (Variables|Default|GetSpellOwner)) (LocalVariables|GetClickedPosition))) :!label _label_2)
            (:LoopBody
              (LocalVariables|SetTargetPlayer (- (LocalVariables|GetTargetPlayer) (LocalVariables|GetDirection)))
              (LocalVariables|SetDistanceParc _index)
              (if (Utilities|Enum|NotEqual(Enum) (.m_typesoftile (.Value (Utilities|Map|Find (Variables|/Game/01_BP/Grid/GridBehaviours.GridBehaviours_C|Getstruct_Tiles (LocalVariables|GetGridManager)) (- (LocalVariables|GetTargetPlayer) (LocalVariables|GetDirection))))) "NewEnumerator6")
                (if (== (.height (.Value (Utilities|Map|Find (Variables|/Game/01_BP/Grid/GridBehaviours.GridBehaviours_C|Getstruct_Tiles (LocalVariables|GetGridManager)) (- (LocalVariables|GetTargetPlayer) (LocalVariables|GetDirection))))) (Variables|/Game/01_BP/03_Character/TopDownCharacter.TopDownCharacter_C|GetPlayerHeight (LocalVariables|GetSpellTarget)))
                  (bind _astop_down_character_3 (Utilities|Casting|CastToTopDownCharacter (.unitonthistile (.Value (Utilities|Map|Find (Variables|/Game/01_BP/Grid/GridBehaviours.GridBehaviours_C|Getstruct_Tiles (LocalVariables|GetGridManager)) (- (LocalVariables|GetTargetPlayer) (LocalVariables|GetDirection))))))
                    (:then
                      (if (!= _astop_down_character_3 (LocalVariables|GetSpellTarget))
                        (Default|ETakeDamage _astop_down_character_3 (/ (CallFunction|GetDamage) 2))
                        (else
                          (Utilities|Casting|CastToBP_Base_Obstacle (.unitonthistile (.Value (Utilities|Map|Find (Variables|/Game/01_BP/Grid/GridBehaviours.GridBehaviours_C|Getstruct_Tiles (LocalVariables|GetGridManager)) (- (LocalVariables|GetTargetPlayer) (LocalVariables|GetDirection))))) :!label _label_3))))
                    (:CastFailed
                      (goto _label_3)))
                  (Transformation|SetActorLocation (LocalVariables|GetSpellTarget) (.m_tiles_worldlocation (.Value (Utilities|Map|Find (Variables|/Game/01_BP/Grid/GridBehaviours.GridBehaviours_C|Getstruct_Tiles (LocalVariables|GetGridManager)) (LocalVariables|GetTargetPlayer)))) false false)
                  (Default|GetUnitonTile (LocalVariables|GetSpellTarget) (LocalVariables|GetTargetPlayer))
                  (LocalVariables|Setdamage (+ (/ (CallFunction|GetDamage) 2) (LocalVariables|Getdamage)))
                  (goto _label_2 Break)
                  (else
                    (if (or (Utilities|Enum|Equal(Enum) (.m_typesoftile (.Value (Utilities|Map|Find (Variables|/Game/01_BP/Grid/GridBehaviours.GridBehaviours_C|Getstruct_Tiles (LocalVariables|GetGridManager)) (- (LocalVariables|GetTargetPlayer) (LocalVariables|GetDirection))))) "NewEnumerator5") (> (.height (.Value (Utilities|Map|Find (Variables|/Game/01_BP/Grid/GridBehaviours.GridBehaviours_C|Getstruct_Tiles (LocalVariables|GetGridManager)) (- (LocalVariables|GetTargetPlayer) (LocalVariables|GetDirection))))) (Variables|/Game/01_BP/03_Character/TopDownCharacter.TopDownCharacter_C|GetPlayerHeight (LocalVariables|GetSpellTarget))))
                      _
                      (else
                        (bind _astop_down_character_4 (Utilities|Casting|CastToTopDownCharacter (.unitonthistile (.Value (Utilities|Map|Find (Variables|/Game/01_BP/Grid/GridBehaviours.GridBehaviours_C|Getstruct_Tiles (LocalVariables|GetGridManager)) (- (LocalVariables|GetTargetPlayer) (LocalVariables|GetDirection))))))
                          (:then
                            (CallFunction|FallEffect0 _astop_down_character_4 (.height (.Value (Utilities|Map|Find (Variables|/Game/01_BP/Grid/GridBehaviours.GridBehaviours_C|Getstruct_Tiles (LocalVariables|GetGridManager)) (- (LocalVariables|GetTargetPlayer) (LocalVariables|GetDirection)))))))
                          (:CastFailed
                            (Utilities|Casting|CastToBP_Base_Obstacle (.unitonthistile (.Value (Utilities|Map|Find (Variables|/Game/01_BP/Grid/GridBehaviours.GridBehaviours_C|Getstruct_Tiles (LocalVariables|GetGridManager)) (- (LocalVariables|GetTargetPlayer) (LocalVariables|GetDirection)))))
                              (:then
                                _)
                              (:CastFailed
                                (Transformation|SetActorLocation (LocalVariables|GetSpellTarget) (.m_tiles_worldlocation (.Value (Utilities|Map|Find (Variables|/Game/01_BP/Grid/GridBehaviours.GridBehaviours_C|Getstruct_Tiles (LocalVariables|GetGridManager)) (- (LocalVariables|GetTargetPlayer) (LocalVariables|GetDirection))))) false false)
                                (Default|GetUnitonTile (LocalVariables|GetSpellTarget) (- (LocalVariables|GetTargetPlayer) (LocalVariables|GetDirection)))
                                (goto _label_2 Break)))))))
                    (LocalVariables|Setdamage (+ (/ (CallFunction|GetDamage) 2) (LocalVariables|Getdamage)))
                    (goto _label_2 Break)))))
            (:Completed
              (Default|ETakeDamage (LocalVariables|GetSpellTarget) (CallFunction|GetDamage) (Variables|Default|GetSpellOwner))
              (Variables|Default|Setm_Cost (+ (Variables|Default|Getm_Cost) (LocalVariables|GetDistanceParc)))
              (Transformation|SetActorLocation (LocalVariables|GetSpellTarget) (.m_tiles_worldlocation (.Value (Utilities|Map|Find (Variables|/Game/01_BP/Grid/GridBehaviours.GridBehaviours_C|Getstruct_Tiles (LocalVariables|GetGridManager)) (+ (LocalVariables|GetTargetPlayer) (LocalVariables|GetDirection))))) false false)
              (Default|GetUnitonTile (LocalVariables|GetSpellTarget) (+ (LocalVariables|GetTargetPlayer) (LocalVariables|GetDirection))))))
        (elif (and (Utilities|Enum|NotEqual(Enum) (.m_typesoftile (.Value (Utilities|Map|Find (Variables|/Game/01_BP/Grid/GridBehaviours.GridBehaviours_C|Getstruct_Tiles (LocalVariables|GetGridManager)) (- (LocalVariables|GetTargetPlayer) (* (LocalVariables|GetDirection) 2.0))))) "NewEnumerator6") (Utilities|Enum|NotEqual(Enum) (.m_typesoftile (.Value (Utilities|Map|Find (Variables|/Game/01_BP/Grid/GridBehaviours.GridBehaviours_C|Getstruct_Tiles (LocalVariables|GetGridManager)) (- (LocalVariables|GetTargetPlayer) (* (LocalVariables|GetDirection) 2.0))))) "NewEnumerator5"))
          (if (== (.height (.Value (Utilities|Map|Find (Variables|/Game/01_BP/Grid/GridBehaviours.GridBehaviours_C|Getstruct_Tiles (LocalVariables|GetGridManager)) (- (LocalVariables|GetTargetPlayer) (* (LocalVariables|GetDirection) 2.0))))) (Variables|/Game/01_BP/03_Character/TopDownCharacter.TopDownCharacter_C|GetPlayerHeight (LocalVariables|GetSpellTarget)))
            (bind _astop_down_character_5 (Utilities|Casting|CastToTopDownCharacter (.unitonthistile (.Value (Utilities|Map|Find (Variables|/Game/01_BP/Grid/GridBehaviours.GridBehaviours_C|Getstruct_Tiles (LocalVariables|GetGridManager)) (- (LocalVariables|GetTargetPlayer) (* (LocalVariables|GetDirection) 2.0))))))
              (:then
                (Default|ETakeDamage _astop_down_character_5 (/ (CallFunction|GetDamage) 2))
                (LocalVariables|Setdamage (+ (/ (CallFunction|GetDamage) 2) (LocalVariables|Getdamage)) :!label _label_4))
              (:CastFailed
                (Utilities|Casting|CastToBP_Base_Obstacle (.unitonthistile (.Value (Utilities|Map|Find (Variables|/Game/01_BP/Grid/GridBehaviours.GridBehaviours_C|Getstruct_Tiles (LocalVariables|GetGridManager)) (- (LocalVariables|GetTargetPlayer) (* (LocalVariables|GetDirection) 2.0)))))
                  (:then
                    (goto _label_4))
                  (:CastFailed
                    (Transformation|SetActorLocation (LocalVariables|GetSpellTarget) (.m_tiles_worldlocation (.Value (Utilities|Map|Find (Variables|/Game/01_BP/Grid/GridBehaviours.GridBehaviours_C|Getstruct_Tiles (LocalVariables|GetGridManager)) (- (LocalVariables|GetTargetPlayer) (* (LocalVariables|GetDirection) 2.0))))) false false :!label _label_5)
                    (Default|GetUnitonTile (LocalVariables|GetSpellTarget) (- (LocalVariables|GetTargetPlayer) (* (LocalVariables|GetDirection) 2.0)))))))
            (else
              (if (> (.height (.Value (Utilities|Map|Find (Variables|/Game/01_BP/Grid/GridBehaviours.GridBehaviours_C|Getstruct_Tiles (LocalVariables|GetGridManager)) (- (LocalVariables|GetTargetPlayer) (* (LocalVariables|GetDirection) 2.0))))) (Variables|/Game/01_BP/03_Character/TopDownCharacter.TopDownCharacter_C|GetPlayerHeight (LocalVariables|GetSpellTarget)))
                _
                (else
                  (Utilities|Casting|CastToTopDownCharacter (.unitonthistile (.Value (Utilities|Map|Find (Variables|/Game/01_BP/Grid/GridBehaviours.GridBehaviours_C|Getstruct_Tiles (LocalVariables|GetGridManager)) (- (LocalVariables|GetTargetPlayer) (* (LocalVariables|GetDirection) 2.0)))))
                    (:then
                      _)
                    (:CastFailed
                      (Utilities|Casting|CastToBP_Base_Obstacle (.unitonthistile (.Value (Utilities|Map|Find (Variables|/Game/01_BP/Grid/GridBehaviours.GridBehaviours_C|Getstruct_Tiles (LocalVariables|GetGridManager)) (- (LocalVariables|GetTargetPlayer) (* (LocalVariables|GetDirection) 2.0)))))
                        (:then
                          _)
                        (:CastFailed
                          (goto _label_5)))))))
              (LocalVariables|Setdamage (+ (/ (CallFunction|GetDamage) 2) (LocalVariables|Getdamage)))))
          (bind _output_get (CallFunction|FallEffect (LocalVariables|GetSpellTarget) (.height (.Value (Utilities|Map|Find (Variables|/Game/01_BP/Grid/GridBehaviours.GridBehaviours_C|Getstruct_Tiles (LocalVariables|GetGridManager)) (- (LocalVariables|GetTargetPlayer) (* (LocalVariables|GetDirection) 2.0)))))))
          (LocalVariables|Setdamage (+ _output_get (LocalVariables|Getdamage)))
          (Default|ETakeDamage (LocalVariables|GetSpellTarget) (LocalVariables|Getdamage)))))
    (:CastFailed
      (goto _label))))

(fn PushAction2
  (params (SpellTarget :type Top%20Down%20Character%20Object%20Reference) (targetTiles :type Vector%202D%20Structure) (grid :type Grid%20Behaviours%20Object%20Reference))
  (bind _damage (CallFunction|GetDamage))
  (LocalVariables|SetTarget SpellTarget)
  (LocalVariables|SetCurrentTiles targetTiles)
  (LocalVariables|SetGridManager grid)
  (if (> (Variables|/Game/01_BP/03_Character/TopDownCharacter.TopDownCharacter_C|GetPlayerHeight (LocalVariables|GetTarget)) (.height (.Value (Utilities|Map|Find (Variables|/Game/01_BP/Grid/GridBehaviours.GridBehaviours_C|Getstruct_Tiles (LocalVariables|GetGridManager)) (LocalVariables|GetCurrentTiles)))))
    (if (== (.unitonthistile (.Value (Utilities|Map|Find (Variables|/Game/01_BP/Grid/GridBehaviours.GridBehaviours_C|Getstruct_Tiles (LocalVariables|GetGridManager)) (LocalVariables|GetCurrentTiles)))) 0)
      (if (> (- (Variables|/Game/01_BP/03_Character/TopDownCharacter.TopDownCharacter_C|GetPlayerHeight (LocalVariables|GetTarget)) (.height (.Value (Utilities|Map|Find (Variables|/Game/01_BP/Grid/GridBehaviours.GridBehaviours_C|Getstruct_Tiles (LocalVariables|GetGridManager)) (LocalVariables|GetCurrentTiles))))) 0)
        (switch int (.height (.Value (Utilities|Map|Find (Variables|/Game/01_BP/Grid/GridBehaviours.GridBehaviours_C|Getstruct_Tiles (LocalVariables|GetGridManager)) (LocalVariables|GetCurrentTiles))))
          (:0
            (return -1 "(X=-1.000000,Y=-1.000000)"))
          (:1
            (LocalVariables|SetFallDamage (/ _damage 2)))
          (:2
            (LocalVariables|SetFallDamage _damage)))
        (CallFunction|GetHeightAction (.height (.Value (Utilities|Map|Find (Variables|/Game/01_BP/Grid/GridBehaviours.GridBehaviours_C|Getstruct_Tiles (LocalVariables|GetGridManager)) (LocalVariables|GetCurrentTiles)))))
        (bind _output_get (LocalVariables|SetFallDamage (LocalVariables|GetFallDamage)))
        (return _output_get (LocalVariables|GetCurrentTiles))
        (else
          (return (/ (CallFunction|GetDamage) 2) (- (LocalVariables|GetCurrentTiles) (Math|Vector2D|Normalize2D (- (LocalVariables|GetCurrentTiles) (Variables|/Game/01_BP/03_Character/TopDownCharacter.TopDownCharacter_C|Getgrid%20Index (Variables|Default|GetSpellOwner))))))))
      (else
        (bind _astop_down_character (Utilities|Casting|CastToTopDownCharacter (.unitonthistile (.Value (Utilities|Map|Find (Variables|/Game/01_BP/Grid/GridBehaviours.GridBehaviours_C|Getstruct_Tiles (LocalVariables|GetGridManager)) (LocalVariables|GetCurrentTiles))))))
        (Default|ETakeDamage _astop_down_character (/ (CallFunction|GetDamage) 2))
        (return 0 (LocalVariables|GetCurrentTiles))))))

(fn ReduceInit
  (params (Direction :type Vector%202D%20Structure))
  (switch int (Math|Float|Truncate (CallFunction|ManhattanDistance Direction (Variables|/Game/01_BP/03_Character/TopDownCharacter.TopDownCharacter_C|Getgrid%20Index (Variables|Default|GetSpellOwner))))
    (:Default
      (LocalVariables|SetcurrentCost (Variables|Default|Getm_Cost)))
    (:0
      (LocalVariables|SetcurrentCost (Variables|Default|Getm_Cost)))
    (:1
      (LocalVariables|SetcurrentCost (Variables|Default|Getm_Cost)))
    (:2
      (LocalVariables|SetcurrentCost 50))
    (:3
      (LocalVariables|SetcurrentCost 60)))
  (Variables|/Game/01_BP/03_Character/TopDownCharacter.TopDownCharacter_C|Setm_Initiative (Variables|Default|GetSpellOwner) (- (Variables|/Game/01_BP/03_Character/TopDownCharacter.TopDownCharacter_C|Getm_Initiative (Variables|Default|GetSpellOwner)) (LocalVariables|GetcurrentCost))))

(fn FallEffect0
  (params (target :type Top%20Down%20Character%20Object%20Reference) (Height :type Integer))
  (switch int (- (Variables|/Game/01_BP/03_Character/TopDownCharacter.TopDownCharacter_C|GetPlayerHeight target) Height)
    (:Default
      _)
    (:0
      _)
    (:1
      (bind _output_get (LocalVariables|SetDamageGiven (+ (CallFunction|GetDamage) (LocalVariables|GetDamageGiven)) :!label _label)))
    (:2
      (if (>= (Variables|/Game/01_BP/03_Character/TopDownCharacter.TopDownCharacter_C|Getm_Initiative target) 100)
        (Variables|/Game/01_BP/03_Character/TopDownCharacter.TopDownCharacter_C|Setm_Initiative target 50)
        (else
          (Variables|/Game/01_BP/03_Character/TopDownCharacter.TopDownCharacter_C|Setm_Initiative target (/ (Variables|/Game/01_BP/03_Character/TopDownCharacter.TopDownCharacter_C|Getm_Initiative target) 2))))
      (Development|PrintString (Utilities|String|ToString(Integer) (Variables|/Game/01_BP/03_Character/TopDownCharacter.TopDownCharacter_C|Getm_Initiative target)))
      (goto _label)))
  (return _output_get))