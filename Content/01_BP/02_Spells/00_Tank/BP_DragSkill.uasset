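; Tank drag spell for a grid-based tactics game that damages another owner's unit and pulls it one tile toward the caster.
; GetReachableTarget uses grid pathfinding within range, keeping only tiles on the caster's row or column as valid targets.
; On a valid cast, DragActionResult moves the victim if the destination is empty, then the spell calls ReduceInit and deselects.
; Collision damage and obstacle debuff logic exists but is unconnected.
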(event EventEUseSpellonTarget
  (params (Grid :type Grid%20Behaviours%20Object%20Reference) (Target%20position :type Vector%202D%20Structure) (SpellOwner :type Top%20Down%20Character%20Object%20Reference))
  (bind _struct_tiles (Variables|/Game/01_BP/Grid/GridBehaviours.GridBehaviours_C|Getstruct_Tiles Grid))
  (bind _value (Utilities|Map|Find _struct_tiles Target%20position))
  (bind (_astop_down_character _bsuccess) (Utilities|Casting|CastToTopDownCharacter (.unitonthistile _value)))
  (if (Utilities|Array|ContainsItem (Variables|Default|GetReachableTarger) Target%20position)
    (if (Math|Boolean|ANDBoolean _bsuccess (Utilities|Enum|NotEqual(Enum) (.m_typesoftile _value) "NewEnumerator5") (Utilities|Enum|NotEqual(Enum) (.m_typesoftile _value) "NewEnumerator6") (Utilities|Enum|NotEqual(Enum) (Variables|/Game/01_BP/03_Character/TopDownCharacter.TopDownCharacter_C|Getm_PawnOwner _astop_down_character) (Variables|/Game/01_BP/03_Character/TopDownCharacter.TopDownCharacter_C|Getm_PawnOwner SpellOwner)))
      (Default|ETakeDamage _astop_down_character (Variables|Default|GetmaxDegats))
      (CallFunction|DragActionResult _astop_down_character SpellOwner Grid)
      (CallFunction|ReduceInit)
      (Default|EDeselectSpeel SpellOwner))))

(fn ConstructionScript
  (|CallParentFunction))

(fn DragActionResult
  (params (Spell%20Target :type Top%20Down%20Character%20Object%20Reference) (Spell%20Caster :type Top%20Down%20Character%20Object%20Reference) (GridManager :type Grid%20Behaviours%20Object%20Reference))
  (LocalVariables|SetTarget Spell%20Target)
  (LocalVariables|SetCaster Spell%20Caster)
  (LocalVariables|SetGrid GridManager)
  (if (== (.unitonthistile (.Value (Utilities|Map|Find (Variables|/Game/01_BP/Grid/GridBehaviours.GridBehaviours_C|Getstruct_Tiles (LocalVariables|GetGrid)) (- (Variables|/Game/01_BP/03_Character/TopDownCharacter.TopDownCharacter_C|Getgrid%20Index (LocalVariables|GetTarget)) (Math|Vector2D|Normalize2D (- (Variables|/Game/01_BP/03_Character/TopDownCharacter.TopDownCharacter_C|Getgrid%20Index (LocalVariables|GetTarget)) (Variables|/Game/01_BP/03_Character/TopDownCharacter.TopDownCharacter_C|Getgrid%20Index (LocalVariables|GetCaster)))))))) 0)
    (Transformation|SetActorLocation (LocalVariables|GetTarget) (.m_tiles_worldlocation (.Value (Utilities|Map|Find (Variables|/Game/01_BP/Grid/GridBehaviours.GridBehaviours_C|Getstruct_Tiles (LocalVariables|GetGrid)) (- (Variables|/Game/01_BP/03_Character/TopDownCharacter.TopDownCharacter_C|Getgrid%20Index (LocalVariables|GetTarget)) (Math|Vector2D|Normalize2D (- (Variables|/Game/01_BP/03_Character/TopDownCharacter.TopDownCharacter_C|Getgrid%20Index (LocalVariables|GetTarget)) (Variables|/Game/01_BP/03_Character/TopDownCharacter.TopDownCharacter_C|Getgrid%20Index (LocalVariables|GetCaster)))))))) false false)
    (Variables|/Game/01_BP/03_Character/TopDownCharacter.TopDownCharacter_C|Setgrid%20Index (LocalVariables|GetTarget) (.m_tiles_index (.Value (Utilities|Map|Find (Variables|/Game/01_BP/Grid/GridBehaviours.GridBehaviours_C|Getstruct_Tiles (LocalVariables|GetGrid)) (- (Variables|/Game/01_BP/03_Character/TopDownCharacter.TopDownCharacter_C|Getgrid%20Index (LocalVariables|GetTarget)) (Math|Vector2D|Normalize2D (- (Variables|/Game/01_BP/03_Character/TopDownCharacter.TopDownCharacter_C|Getgrid%20Index (LocalVariables|GetTarget)) (Variables|/Game/01_BP/03_Character/TopDownCharacter.TopDownCharacter_C|Getgrid%20Index (LocalVariables|GetCaster)))))))))))

(fn GetReachableTarget
  (params (Origin%20Index :type Vector%202D%20Structure) (Distance :type Integer) (Grid :type Grid%20Behaviours%20Object%20Reference))
  (bind _spellowner (Variables|Default|GetSpellOwner))
  (bind _grid_index (Variables|/Game/01_BP/03_Character/TopDownCharacter.TopDownCharacter_C|Getgrid%20Index _spellowner))
  (LocalVariables|SetFirstIndex Origin%20Index)
  (LocalVariables|Setm_Distance Distance)
  (bind _keys (Utilities|Map|Keys (Variables|/Game/01_BP/Grid/GridBehaviours.GridBehaviours_C|Getstruct_Tiles Grid)))
  (bind _array_element (Utilities|Array|ForEachLoopwithBreak _keys :!label _label)
    (:LoopBody
      (bind _output_get (LocalVariables|SetTargetIndex _array_element))
      (if (Math|Boolean|ORBoolean (!= (.unitonthistile (.Value (Utilities|Map|Find (Variables|/Game/01_BP/Grid/GridBehaviours.GridBehaviours_C|Getstruct_Tiles Grid) _output_get))) 0) (Utilities|Enum|Equal(Enum) (.m_typesoftile (.Value (Utilities|Map|Find (Variables|/Game/01_BP/Grid/GridBehaviours.GridBehaviours_C|Getstruct_Tiles Grid) _output_get))) "NewEnumerator6") (Utilities|Enum|Equal(Enum) (.m_typesoftile (.Value (Utilities|Map|Find (Variables|/Game/01_BP/Grid/GridBehaviours.GridBehaviours_C|Getstruct_Tiles Grid) _output_get))) "NewEnumerator5") (> (Default|GetEstimatedCosttoTarget Grid (LocalVariables|GetFirstIndex) (LocalVariables|GetTargetIndex)) (LocalVariables|Getm_Distance)))
        (goto _label Break)))
    (:Completed
      (bind _reachable_tiles (Default|FindPathtoTarget Grid (LocalVariables|GetFirstIndex) (LocalVariables|GetTargetIndex) (LocalVariables|Getm_Distance) true false false))
      (for _array_element_2 _reachable_tiles
        (if (or (== (.X (Math|Vector2D|BreakVector2D _array_element_2)) (.x _grid_index)) (== (.y _grid_index) (.Y (Math|Vector2D|BreakVector2D _array_element_2))))
          (Utilities|Array|AddUnique (Variables|Default|GetReachableTarger) _array_element_2)))
      (return (Variables|Default|GetReachableTarger)))))