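; BP_ProtectSpell is the tank's protection spell, which puts its caster into a protected state.
; When used, it casts the owner to Tank_Character and sets IsProtection, or plays a failure sound otherwise.
; PlaySpellAnimation picks the shield montage matching the black or brown cow variant.
; On montage completion, it calls ReduceInit, resets CurrentDistance, plays the FMOD spell sound and deselects the spell.
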(event EventBeginPlay
  (|CallParentFunction) ; This node is disabled and will not be called.\nDrag off pins to build functionality.
)

(event EventEUseSpellonTarget
  (params (Grid :type Grid%20Behaviours%20Object%20Reference) (Target%20position :type Vector%202D%20Structure) (SpellOwner :type Top%20Down%20Character%20Object%20Reference))
  (bind _astank_character (Utilities|Casting|CastToTank_Character SpellOwner)
    (:then
      (Variables|/Game/01_BP/03_Character/Tank_Character.Tank_Character_C|SetIsProtection _astank_character true)
      (bind (_targetmesh _animmotagetouse1) (CallFunction|PlaySpellAnimation))
      (Animation|Montage|PlayMontage (Variables|/Script/Engine.Character|GetMesh _targetmesh) _animmotagetouse1
        (:OnCompleted
          (CallFunction|ReduceInit)
          (Variables|Default|SetcurrentDistance (Variables|Default|Getm_Distances))
          (Class|FMODAudioComponent|Play (Variables|Default|GetAttaque_FMODAudio))
          (Default|EDeselectSpeel SpellOwner))))
    (:CastFailed
      (Class|FMODAudioComponent|Play (Variables|Default|GetCantAttaque_FMODAudio)))))

(fn ConstructionScript
  (|CallParentFunction))

(fn PlaySpellAnimation
  (bind _astank_character_cow_black (Utilities|Casting|CastToTank_Character_Cow_Black (Variables|Default|GetSpellOwner))
    (:then
      (LocalVariables|SetTarget _astank_character_cow_black)
      (LocalVariables|SetAnimToUse "/Game/06_Animation/Anim_Dark/Cow/CowDark_Shield_AM.CowDark_Shield_AM"))
    (:CastFailed
      (bind _astank_character_cow_brown (Utilities|Casting|CastToTank_Character_Cow_Brown (Variables|Default|GetSpellOwner)))
      (LocalVariables|SetTarget _astank_character_cow_brown)
      (LocalVariables|SetAnimToUse "/Game/06_Animation/Anim_Brown/Cow/CowBrown_Shield_AM.CowBrown_Shield_AM")))
  (return (LocalVariables|GetTarget) (LocalVariables|GetAnimToUse)))