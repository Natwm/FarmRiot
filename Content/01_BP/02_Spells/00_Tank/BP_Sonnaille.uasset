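; Tank spell Sonnaille, which links friendly units in its target area to the casting Tank.
; On preview it builds targets from attackable tiles refined by the grid's around-unit query, then toggles their highlight; a caster at height 2 enables CanGetArround.
; On use it sets TankIntoSonnaille on same-owner units in those tiles, deselects the spell and plays FMOD audio.
; The height filter function is never called.
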(event EventEShowTilesTargetedbySpell
  (params (Origin%20Index :type Vector%202D%20Structure) (Grid :type Grid%20Behaviours%20Object%20Reference) (Show%20Tiles :type Boolean))
  (if (== (Variables|/Game/01_BP/03_Character/TopDownCharacter.TopDownCharacter_C|GetPlayerHeight (Variables|Default|GetSpellOwner)) 2)
    (Variables|Default|SetCanGetArround true)
    (Variables|Default|Setm_Distances 3))
  (if (> (Utilities|Array|Length (Variables|Default|GetReachableTarget)) 0)
    (Default|HighlightAttackableTiles Grid (Variables|Default|GetReachableTarget) false)
    (Utilities|Array|Clear (Variables|Default|GetReachableTarget))
    (Utilities|Array|Clear (Variables|Default|GetAttackableTiles))
    (Utilities|Array|Clear (Variables|Default|GetUnAttackableTiles)))
  (bind _newlocalvar_01 (CallFunction|GetAttackableTiles Origin%20Index Grid))
  (bind _output_get (Variables|Default|SetReachableTarget _newlocalvar_01))
  (bind _tilesarroundtheplayer (Default|GetTileArround Grid _output_get (Variables|/Game/01_BP/03_Character/TopDownCharacter.TopDownCharacter_C|Getgrid%20Index (Variables|Default|GetSpellOwner))))
  (Variables|Default|SetReachableTarget _tilesarroundtheplayer)
  (Default|HighlightAttackableTiles Grid (Variables|Default|GetReachableTarget) Show%20Tiles)
  (Variables|Default|Setm_Distances 1))

(event EventEUseSpellonTarget
  (params (Grid :type Grid%20Behaviours%20Object%20Reference) (Target%20position :type Vector%202D%20Structure) (SpellOwner :type Top%20Down%20Character%20Object%20Reference))
  (for _array_element (Variables|Default|GetReachableTarget)
    (bind _astop_down_character (Utilities|Casting|CastToTopDownCharacter (.unitonthistile (.Value (Utilities|Map|Find (Variables|/Game/01_BP/Grid/GridBehaviours.GridBehaviours_C|Getstruct_Tiles Grid) _array_element)))))
    (if (Utilities|Enum|Equal(Enum) (Variables|/Game/01_BP/03_Character/TopDownCharacter.TopDownCharacter_C|Getm_PawnOwner _astop_down_character) (Variables|/Game/01_BP/03_Character/TopDownCharacter.TopDownCharacter_C|Getm_PawnOwner SpellOwner))
      (bind _astank_character (Utilities|Casting|CastToTank_Character SpellOwner))
      (Variables|/Game/01_BP/03_Character/TopDownCharacter.TopDownCharacter_C|SetTankIntoSonnaille _astop_down_character _astank_character)))
  (Variables|Default|Setm_Distances 1)
  (Default|EDeselectSpeel SpellOwner)
  (Class|FMODAudioComponent|Play (Variables|Default|GetAttaque_FMODAudio)))

(fn ConstructionScript
  (|CallParentFunction))

(fn CanAffectThisbyHeight
  (params (Array :type Array%20of%20Vector%202D%20Structures) (self2 :type Grid%20Behaviours%20Object%20Reference))
  (for _array_element Array
    (if (not (< (.height (.Value (Utilities|Map|Find (Variables|/Game/01_BP/Grid/GridBehaviours.GridBehaviours_C|Getstruct_Tiles self2) _array_element))) (Variables|/Game/01_BP/03_Character/TopDownCharacter.TopDownCharacter_C|GetPlayerHeight (Variables|Default|GetSpellOwner))))
      (Utilities|Array|RemoveItem (Variables|Default|GetReachableTarget) _array_element))))