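; Turkey egg spell for the grid-based game, cast on a free, valid tile within reach.
; If the caster stands higher than the target it damages units on tiles around it; otherwise it spawns a BP_Fiente registered on that tile with damage and owner.
; CanSpawnAnEgg caps these at two per player by counting existing actors.
; A successful cast plays the black or brown turkey montage, then deselects the spell.
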(event EventEUseSpellonTarget
  (params (Grid :type Grid%20Behaviours%20Object%20Reference) (Target%20position :type Vector%202D%20Structure) (SpellOwner :type Top%20Down%20Character%20Object%20Reference))
  (bind _struct_tiles (Variables|/Game/01_BP/Grid/GridBehaviours.GridBehaviours_C|Getstruct_Tiles Grid))
  (bind _value (Utilities|Map|Find _struct_tiles Target%20position))
  (if (Utilities|Array|ContainsItem (Variables|Default|GetReachableTarget) Target%20position)
    (if (Math|Boolean|ANDBoolean (not (.bSuccess (Utilities|Casting|CastToTopDownCharacter (.unitonthistile _value)))) (Utilities|Enum|NotEqual(Enum) (.m_typesoftile _value) "NewEnumerator5") (Utilities|Enum|NotEqual(Enum) (.m_typesoftile _value) "NewEnumerator6") (== (.isfruit _value) 0) (== (.isspecialtile _value) 0))
      (if (> (- (Variables|/Game/01_BP/03_Character/TopDownCharacter.TopDownCharacter_C|GetPlayerHeight (Variables|Default|GetSpellOwner)) (.height _value)) 0)
        (bind _tilesarroundtheplayer (Default|GetTileArround Grid (Variables|Default|GetReachableTarget) (Variables|/Game/01_BP/03_Character/TopDownCharacter.TopDownCharacter_C|Getgrid%20Index (Variables|Default|GetSpellOwner))))
        (for _array_element _tilesarroundtheplayer
          (bind _astop_down_character (Utilities|Casting|CastToTopDownCharacter (.unitonthistile (.Value (Utilities|Map|Find (Variables|/Game/01_BP/Grid/GridBehaviours.GridBehaviours_C|Getstruct_Tiles Grid) _array_element)))))
          (CallFunction|AffectDamage _astop_down_character (.height (.Value (Utilities|Map|Find (Variables|/Game/01_BP/Grid/GridBehaviours.GridBehaviours_C|Getstruct_Tiles Grid) _array_element)))))
        (CallFunction|ReduceInit :!label _label)
        (Variables|Default|SetcurrentDistance (Variables|Default|Getm_Distances))
        (bind (_targetmesh _animmotagetouse1) (CallFunction|PlaySpellAnimation))
        (Animation|Montage|PlayMontage (Variables|/Script/Engine.Character|GetMesh _targetmesh) _animmotagetouse1
          (:OnCompleted
            (Default|EDeselectSpeel SpellOwner)
            (Class|FMODAudioComponent|Play (Variables|Default|GetAttaque_FMODAudio))))
        (else
          (bind _returnvalue (CallFunction|CanSpawnAnEgg))
          (if _returnvalue
            (bind _returnvalue_2 (Game|SpawnActorfromClass "/Game/01_BP/06_SpawnObject/BP_Fiente.BP_Fiente_C" (Math|Transform|MakeTransform (.m_tiles_worldlocation _value) "0, 0, 0" "1,1,1") "Undefined" 0 0))
            (CallFunction|SetUnitonATile Grid Target%20position _returnvalue_2)
            (goto _label))))
      (else
        (Class|FMODAudioComponent|Play (Variables|Default|GetCantAttaque_FMODAudio))))))

(fn ConstructionScript
  (|CallParentFunction))

(fn SetUnitonATile
  (params (Grid :type Grid%20Behaviours%20Object%20Reference) (target :type Vector%202D%20Structure) (Fiente :type BP%20Fiente%20Object%20Reference))
  (LocalVariables|SetGridManager Grid)
  (LocalVariables|SetTargetVector2 target)
  (LocalVariables|SetFienteBP Fiente)
  (Utilities|Map|Add (Variables|/Game/01_BP/Grid/GridBehaviours.GridBehaviours_C|Getstruct_Tiles (LocalVariables|GetGridManager)) (LocalVariables|GetTargetVector2) (Utilities|Struct|MakeTiles_Struct (.tileactor (.Value (Utilities|Map|Find (Variables|/Game/01_BP/Grid/GridBehaviours.GridBehaviours_C|Getstruct_Tiles (LocalVariables|GetGridManager)) (LocalVariables|GetTargetVector2)))) 0 (.tilecost (.Value (Utilities|Map|Find (Variables|/Game/01_BP/Grid/GridBehaviours.GridBehaviours_C|Getstruct_Tiles (LocalVariables|GetGridManager)) (LocalVariables|GetTargetVector2)))) (.m_typesoftile (.Value (Utilities|Map|Find (Variables|/Game/01_BP/Grid/GridBehaviours.GridBehaviours_C|Getstruct_Tiles (LocalVariables|GetGridManager)) (LocalVariables|GetTargetVector2)))) (.m_tiles_worldlocation (.Value (Utilities|Map|Find (Variables|/Game/01_BP/Grid/GridBehaviours.GridBehaviours_C|Getstruct_Tiles (LocalVariables|GetGridManager)) (LocalVariables|GetTargetVector2)))) (.m_tiles_index (.Value (Utilities|Map|Find (Variables|/Game/01_BP/Grid/GridBehaviours.GridBehaviours_C|Getstruct_Tiles (LocalVariables|GetGridManager)) (LocalVariables|GetTargetVector2)))) (.finalcost (.Value (Utilities|Map|Find (Variables|/Game/01_BP/Grid/GridBehaviours.GridBehaviours_C|Getstruct_Tiles (LocalVariables|GetGridManager)) (LocalVariables|GetTargetVector2)))) (.costfromstart (.Value (Utilities|Map|Find (Variables|/Game/01_BP/Grid/GridBehaviours.GridBehaviours_C|Getstruct_Tiles (LocalVariables|GetGridManager)) (LocalVariables|GetTargetVector2)))) (.estimatedcosttotarget (.Value (Utilities|Map|Find (Variables|/Game/01_BP/Grid/GridBehaviours.GridBehaviours_C|Getstruct_Tiles (LocalVariables|GetGridManager)) (LocalVariables|GetTargetVector2)))) (.previoustiles (.Value (Utilities|Map|Find (Variables|/Game/01_BP/Grid/GridBehaviours.GridBehaviours_C|Getstruct_Tiles (LocalVariables|GetGridManager)) (LocalVariables|GetTargetVector2)))) (.height (.Value (Utilities|Map|Find (Variables|/Game/01_BP/Grid/GridBehaviours.GridBehaviours_C|Getstruct_Tiles (LocalVariables|GetGridManager)) (LocalVariables|GetTargetVector2)))) (.isfruit (.Value (Utilities|Map|Find (Variables|/Game/01_BP/Grid/GridBehaviours.GridBehaviours_C|Getstruct_Tiles (LocalVariables|GetGridManager)) (LocalVariables|GetTargetVector2)))) (.isspecialtile (.Value (Utilities|Map|Find (Variables|/Game/01_BP/Grid/GridBehaviours.GridBehaviours_C|Getstruct_Tiles (LocalVariables|GetGridManager)) (LocalVariables|GetTargetVector2))))))
  (Variables|/Game/01_BP/07_Obstacles/BP_Base_Obstacle.BP_Base_Obstacle_C|SetGrid%20Index (LocalVariables|GetFienteBP) (LocalVariables|GetTargetVector2))
  (Utilities|Map|Add (Variables|/Game/01_BP/Grid/GridBehaviours.GridBehaviours_C|Getstruct_Tiles (LocalVariables|GetGridManager)) (LocalVariables|GetTargetVector2) (Utilities|Struct|MakeTiles_Struct (.tileactor (.Value (Utilities|Map|Find (Variables|/Game/01_BP/Grid/GridBehaviours.GridBehaviours_C|Getstruct_Tiles (LocalVariables|GetGridManager)) (LocalVariables|GetTargetVector2)))) (LocalVariables|GetFienteBP) (.tilecost (.Value (Utilities|Map|Find (Variables|/Game/01_BP/Grid/GridBehaviours.GridBehaviours_C|Getstruct_Tiles (LocalVariables|GetGridManager)) (LocalVariables|GetTargetVector2)))) "NewEnumerator0" (.m_tiles_worldlocation (.Value (Utilities|Map|Find (Variables|/Game/01_BP/Grid/GridBehaviours.GridBehaviours_C|Getstruct_Tiles (LocalVariables|GetGridManager)) (LocalVariables|GetTargetVector2)))) (.m_tiles_index (.Value (Utilities|Map|Find (Variables|/Game/01_BP/Grid/GridBehaviours.GridBehaviours_C|Getstruct_Tiles (LocalVariables|GetGridManager)) (LocalVariables|GetTargetVector2)))) (.finalcost (.Value (Utilities|Map|Find (Variables|/Game/01_BP/Grid/GridBehaviours.GridBehaviours_C|Getstruct_Tiles (LocalVariables|GetGridManager)) (LocalVariables|GetTargetVector2)))) (.costfromstart (.Value (Utilities|Map|Find (Variables|/Game/01_BP/Grid/GridBehaviours.GridBehaviours_C|Getstruct_Tiles (LocalVariables|GetGridManager)) (LocalVariables|GetTargetVector2)))) (.estimatedcosttotarget (.Value (Utilities|Map|Find (Variables|/Game/01_BP/Grid/GridBehaviours.GridBehaviours_C|Getstruct_Tiles (LocalVariables|GetGridManager)) (LocalVariables|GetTargetVector2)))) (.previoustiles (.Value (Utilities|Map|Find (Variables|/Game/01_BP/Grid/GridBehaviours.GridBehaviours_C|Getstruct_Tiles (LocalVariables|GetGridManager)) (LocalVariables|GetTargetVector2)))) (.height (.Value (Utilities|Map|Find (Variables|/Game/01_BP/Grid/GridBehaviours.GridBehaviours_C|Getstruct_Tiles (LocalVariables|GetGridManager)) (LocalVariables|GetTargetVector2)))) (.isfruit (.Value (Utilities|Map|Find (Variables|/Game/01_BP/Grid/GridBehaviours.GridBehaviours_C|Getstruct_Tiles (LocalVariables|GetGridManager)) (LocalVariables|GetTargetVector2)))) (.isspecialtile (.Value (Utilities|Map|Find (Variables|/Game/01_BP/Grid/GridBehaviours.GridBehaviours_C|Getstruct_Tiles (LocalVariables|GetGridManager)) (LocalVariables|GetTargetVector2))))))
  (Variables|/Game/01_BP/06_SpawnObject/BP_Fiente.BP_Fiente_C|SetDamage (LocalVariables|GetFienteBP) (Variables|Default|GetmaxDegats))
  (Variables|/Game/01_BP/06_SpawnObject/BP_Fiente.BP_Fiente_C|SetPoopOwner (LocalVariables|GetFienteBP) (Variables|/Game/01_BP/03_Character/TopDownCharacter.TopDownCharacter_C|Getm_PawnOwner (Variables|Default|GetSpellOwner))))

(fn PlaySpellAnimation
  (bind _ascontrol_character_turkey_black (Utilities|Casting|CastToControl_Character_Turkey_Black (Variables|Default|GetSpellOwner))
    (:then
      (LocalVariables|SetTarget _ascontrol_character_turkey_black)
      (LocalVariables|SetAnimToUse "/Game/06_Animation/Anim_Dark/Dinde/DindeDark_Oeuf_AM.DindeDark_Oeuf_AM"))
    (:CastFailed
      (bind _ascontrol_character_turkey_brown (Utilities|Casting|CastToControl_Character_Turkey_Brown (Variables|Default|GetSpellOwner)))
      (LocalVariables|SetTarget _ascontrol_character_turkey_brown)
      (LocalVariables|SetAnimToUse "/Game/06_Animation/Anim_Brown/Dinde/DindeBrown_Oeuf_AM.DindeBrown_Oeuf_AM")))
  (return (LocalVariables|GetTarget) (LocalVariables|GetAnimToUse)))

(fn CanSpawnAnEgg
  (bind _outactors (Actor|GetAllActorsOfClass "/Game/01_BP/06_SpawnObject/BP_Fiente.BP_Fiente_C"))
  (for _array_element _outactors
    (switch Utilities|FlowControl|Switch|SwitchonOwner (Variables|/Game/01_BP/06_SpawnObject/BP_Fiente.BP_Fiente_C|GetPoopOwner _array_element)
      (:NewEnumerator0
        (Math|Integer|IncrementInt (LocalVariables|GetAmountOfPlayer1)))
      (:NewEnumerator1
        (Math|Integer|IncrementInt (LocalVariables|GetAmountOfPlayer2)))))
  (switch Utilities|FlowControl|Switch|SwitchonOwner (Variables|/Game/01_BP/03_Character/TopDownCharacter.TopDownCharacter_C|Getm_PawnOwner (Variables|Default|GetSpellOwner))
    (:NewEnumerator0
      (LocalVariables|SetReturn (== (LocalVariables|GetAmountOfPlayer1) 2)))
    (:NewEnumerator1
      (LocalVariables|SetReturn (== (LocalVariables|GetAmountOfPlayer2) 2))))
  (Development|PrintString (Utilities|String|ToString(Boolean) (not (LocalVariables|GetReturn))))
  (return (not (LocalVariables|GetReturn))))