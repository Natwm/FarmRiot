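; BP_ProtectSpell is a spell Blueprint that puts a Tank_Character into a protection state.
; On EUseSpellonTarget it casts the spell owner to Tank_Character, stopping if that fails, and sets its IsProtection flag.
; It then calls ReduceInit with a zero vector, sets CurrentDistance to MDistances and plays the attack FMOD audio.
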(event EventBeginPlay
  (|CallParentFunction) ; This node is disabled and will not be called.\nDrag off pins to build functionality.
)

(event EventEUseSpellonTarget
  (params (Grid :type Grid%20Behaviours%20Object%20Reference) (Target%20position :type Vector%202D%20Structure) (SpellOwner :type Top%20Down%20Character%20Object%20Reference))
  (bind _astank_character (Utilities|Casting|CastToTank_Character SpellOwner))
  (Variables|/Game/01_BP/03_Character/Tank_Character.Tank_Character_C|SetIsProtection _astank_character true)
  (CallFunction|ReduceInit)
  (Variables|Default|SetcurrentDistance (Variables|Default|Getm_Distances))
  (Class|FMODAudioComponent|Play (Variables|Default|GetAttaque_FMODAudio)))

(fn ConstructionScript
  (|CallParentFunction))