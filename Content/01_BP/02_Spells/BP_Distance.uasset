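; BP_Distance is the distance spell for the turkey characters, supplying their spell image and animation.
; It implements GetImageToDisplay and PlaySpellAnimation by casting SpellOwner to the Black or Brown turkey.
; The matching variant selects a black or brown feather texture, plus the target character and distance montage returned to the caller.
; The construction script only calls its parent, and no projectile or damage logic is defined here.
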(fn ConstructionScript
  (|CallParentFunction))

(fn GetImagetoDisplay
  (bind _spellowner (Variables|Default|GetSpellOwner))
  (Utilities|Casting|CastToControl_Character_Turkey_Black _spellowner
    (:then
      (LocalVariables|SetTexture%20to%20display "/Game/07_UI/sort_plume_noir.sort_plume_noir"))
    (:CastFailed
      (Utilities|Casting|CastToControl_Character_Turkey_Brown _spellowner)
      (LocalVariables|SetTexture%20to%20display "/Game/07_UI/sort_plume_marron.sort_plume_marron")))
  (return (LocalVariables|GetTexture%20to%20display)))

(fn PlaySpellAnimation
  (bind _ascontrol_character_turkey_black (Utilities|Casting|CastToControl_Character_Turkey_Black (Variables|Default|GetSpellOwner))
    (:then
      (LocalVariables|SetTarget _ascontrol_character_turkey_black)
      (LocalVariables|SetAnimMotageToUse "/Game/06_Animation/Anim_Dark/Dinde/DindeDark_Distance_AM.DindeDark_Distance_AM"))
    (:CastFailed
      (bind _ascontrol_character_turkey_brown (Utilities|Casting|CastToControl_Character_Turkey_Brown (Variables|Default|GetSpellOwner)))
      (LocalVariables|SetTarget _ascontrol_character_turkey_brown)
      (LocalVariables|SetAnimMotageToUse "/Game/06_Animation/Anim_Brown/Dinde/DindeBrown_Distance_AM.DindeBrown_Distance_AM")))
  (return (LocalVariables|GetTarget) (LocalVariables|GetAnimMotageToUse)))