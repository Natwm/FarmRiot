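; BP_BasicSpell is a grid tactics attack spell that highlights targetable tiles and damages the chosen unit.
; Targeting gathers tiles within Manhattan range, filtered by height, then uses grid pathing and line traces to mark blocked ones unless it passes through walls.
; Casting rolls height-adjusted damage on characters, or flat maximum on BP_Fiente, then deducts initiative cost.
; Owners at height 2 gain range by incrementing MDistances on display, reverted only after hitting a character.
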(event Custom|E_UseSpellOnTarget
  (params (Grid :type Grid%20Behaviours%20Object%20Reference) (Target%20position :type Vector%202D%20Structure) (SpellOwner :type Top%20Down%20Character%20Object%20Reference))
  (bind _struct_tiles (Variables|/Game/01_BP/Grid/GridBehaviours.GridBehaviours_C|Getstruct_Tiles Grid))
  (bind _value (Utilities|Map|Find _struct_tiles Target%20position))
  (if (and (Utilities|Array|ContainsItem (Variables|Liste|GetAttackableTiles) Target%20position) (not (Utilities|Array|ContainsItem (Variables|Liste|GetUnAttackableTiles) Target%20position)))
    (if (Math|Boolean|ANDBoolean (CallFunction|IsATargetableUnit (.unitonthistile _value)) (Utilities|Enum|NotEqual(Enum) (.m_typesoftile _value) "NewEnumerator5") (Utilities|Enum|NotEqual(Enum) (.m_typesoftile _value) "NewEnumerator6"))
      (Utilities|Casting|CastToTopDownCharacter (.unitonthistile _value)
        (:then
          (CallFunction|AffectDamage 0 (.height _value))
          (if (== (Variables|/Game/01_BP/03_Character/TopDownCharacter.TopDownCharacter_C|GetPlayerHeight (Variables|Default|GetSpellOwner)) 2)
            (Math|Integer|DecrementInt (Variables|Value|Getm_Distances)
              (:%20%20
                _))))
        (:CastFailed
          (bind _asbp_fiente (Utilities|Casting|CastToBP_Fiente (.unitonthistile _value)))
          (Default|ETakeDamage _asbp_fiente (Variables|Value|GetmaxDegats))))
      (CallFunction|ReduceInit)
      (Default|EDeselectSpeel SpellOwner)
      (Class|FMODAudioComponent|Play (Variables|Default|GetAttaque_FMODAudio))
      (else
        (Class|FMODAudioComponent|Play (Variables|Default|GetCantAttaque_FMODAudio) :!label _label)))
    (else
      (goto _label))))

(event Custom|E_ShowTilesTargetedBySpell
  (params (Origin%20Index :type Vector%202D%20Structure) (Grid :type Grid%20Behaviours%20Object%20Reference) (Show%20Tiles :type Boolean))
  (if (== (Variables|/Game/01_BP/03_Character/TopDownCharacter.TopDownCharacter_C|GetPlayerHeight (Variables|Default|GetSpellOwner)) 2)
    (Math|Integer|IncrementInt (Variables|Value|Getm_Distances)
      (:%20%20
        _)))
  (if (> (Utilities|Array|Length (Variables|Liste|GetReachableTarget)) 0)
    (Default|HighlightAttackableTiles Grid (Variables|Liste|GetReachableTarget) false)
    (Utilities|Array|Clear (Variables|Liste|GetAttackableTiles))
    (Utilities|Array|Clear (Variables|Liste|GetUnAttackableTiles))
    (Utilities|Array|Clear (Variables|Liste|GetReachableTarget)))
  (bind _newlocalvar_01 (CallFunction|GetAttackableTiles Origin%20Index Grid))
  (bind _reachablestargets (CallFunction|GetReachableTargetatMinimumDistances _newlocalvar_01 Origin%20Index))
  (Variables|Liste|SetReachableTarget _reachablestargets)
  (bind _reachable_tiles (Default|GetPossibleTargetIndex Grid (Variables|/Game/01_BP/03_Character/TopDownCharacter.TopDownCharacter_C|Getgrid%20Index (Variables|Default|GetSpellOwner)) (Variables|Value|Getm_Distances)))
  (if (not (Variables|flag|Getm_PassThroughWalls))
    (for _array_element (Variables|Liste|GetReachableTarget)
      (if (Utilities|Array|ContainsItem _reachable_tiles _array_element)
        (Utilities|Array|AddUnique (Variables|Liste|GetAttackableTiles) _array_element)
        (else
          (Utilities|Array|AddUnique (Variables|Liste|GetUnAttackableTiles) _array_element))))
    (else
      (Variables|Liste|SetAttackableTiles (Variables|Liste|GetReachableTarget))))
  (Default|HighlightAttackableTiles Grid (Variables|Liste|GetAttackableTiles) Show%20Tiles)
  (CallFunction|AddUntargatableTiles Grid (Variables|Liste|GetReachableTarget))
  (Default|HighlighUnAttackableTiles Grid (Variables|Liste|GetUnAttackableTiles) Show%20Tiles))

(event EventBeginPlay
  (Variables|Value|SetCurrentMinDamage (Variables|Value|GetminDegats))
  (Variables|Value|SetCurrentMaxDamage (Variables|Value|GetmaxDegats)))

(fn ConstructionScript)

(fn GetReachableTarget
  (params (Origin%20Index :type Vector%202D%20Structure) (Distance :type Integer) (Grid :type Grid%20Behaviours%20Object%20Reference))
  (LocalVariables|SetFirstIndex Origin%20Index)
  (LocalVariables|Setm_Distance Distance)
  (bind _keys (Utilities|Map|Keys (Variables|/Game/01_BP/Grid/GridBehaviours.GridBehaviours_C|Getstruct_Tiles Grid)))
  (bind _array_element (Utilities|Array|ForEachLoopwithBreak _keys :!label _label)
    (:LoopBody
      (bind _output_get (LocalVariables|SetTargetIndex _array_element))
      (if (Math|Boolean|ORBoolean (!= (.unitonthistile (.Value (Utilities|Map|Find (Variables|/Game/01_BP/Grid/GridBehaviours.GridBehaviours_C|Getstruct_Tiles Grid) _output_get))) 0) (Utilities|Enum|Equal(Enum) (.m_typesoftile (.Value (Utilities|Map|Find (Variables|/Game/01_BP/Grid/GridBehaviours.GridBehaviours_C|Getstruct_Tiles Grid) _output_get))) "NewEnumerator6") (Utilities|Enum|Equal(Enum) (.m_typesoftile (.Value (Utilities|Map|Find (Variables|/Game/01_BP/Grid/GridBehaviours.GridBehaviours_C|Getstruct_Tiles Grid) _output_get))) "NewEnumerator5") (> (Default|GetEstimatedCosttoTarget Grid (LocalVariables|GetFirstIndex) (LocalVariables|GetTargetIndex)) (LocalVariables|Getm_Distance)))
        (goto _label Break)))
    (:Completed
      (bind _reachable_tiles (Default|FindPathtoTarget Grid (LocalVariables|GetFirstIndex) (LocalVariables|GetTargetIndex) (LocalVariables|Getm_Distance) true (Variables|flag|Getm_PassThroughWalls) true))
      (return _reachable_tiles))))

(fn GetAttackableTiles
  (params (NewParam :type Vector%202D%20Structure) (grid :type Grid%20Behaviours%20Object%20Reference))
  (bind _newlocalvar_0 (LocalVariables|GetNewLocalVar_0))
  (bind _m_distances (Variables|Value|Getm_Distances))
  (bind _m_distances_2 (Variables|Value|Getm_Distances))
  (for _index (range (* _m_distances_2 -1) _m_distances_2)
    (for _index_2 (range (* _m_distances -1) _m_distances)
      (if (.ReturnValue (CallFunction|DoesThisTilesIsCorrect NewParam _index _index_2 grid))
        (Utilities|Array|AddUnique (LocalVariables|GetNewLocalVar_0) (.ValidPosition (CallFunction|DoesThisTilesIsCorrect NewParam _index _index_2 grid))))))
  (CallFunction|CanAccestoThisTIlewithRayCast _newlocalvar_0 grid)
  (return _newlocalvar_0))

(fn ReduceInit
  (params (Direction :type Vector%202D%20Structure))
  (Variables|/Game/01_BP/03_Character/TopDownCharacter.TopDownCharacter_C|Setm_Initiative (Variables|Default|GetSpellOwner) (- (Variables|/Game/01_BP/03_Character/TopDownCharacter.TopDownCharacter_C|Getm_Initiative (Variables|Default|GetSpellOwner)) (Variables|Value|Getm_Cost))))

(fn GetDirection
  (params (Target :type Vector%202D%20Structure) (Caster :type Vector%202D%20Structure))
  (return (+ Target (Math|Vector2D|Normalize2D (- Target Caster)))))

(fn GetReachableTargetatMinimumDistances
  (params (Targets :type Array%20of%20Vector%202D%20Structures) (unitPos :type Vector%202D%20Structure))
  (for _array_element Targets
    (if (> (Math|Float|Round (Class|KismetMathLibrary|DistanceSquared2D _array_element unitPos)) (Variables|Value|GetMinDistance))
      (Utilities|Array|AddUnique (LocalVariables|GetTiles) _array_element)))
  (return (LocalVariables|GetTiles)))

(fn DoesThisTilesIsCorrect
  (params (InVec :type Vector%202D%20Structure) (X :type Integer) (Y :type Integer) (grid :type Grid%20Behaviours%20Object%20Reference))
  (bind _returnvalue (Math|Conversions|ToFloat(Integer) X))
  (bind _returnvalue_2 (Math|Conversions|ToFloat(Integer) Y))
  (bind (_x _y) (Math|Vector2D|BreakVector2D InVec))
  (bind _struct_tiles (Variables|/Game/01_BP/Grid/GridBehaviours.GridBehaviours_C|Getstruct_Tiles grid))
  (bind _spellowner (Variables|Default|GetSpellOwner))
  (bind _isaffectbyheight (Variables|flag|GetIsAffectByHeight))
  (bind _mindistance (Variables|Value|GetMinDistance))
  (bind _m_distances (Variables|Value|Getm_Distances))
  (bind _canattaquebellow (Variables|Flag|GetCanAttaqueBellow))
  (bind _m_passthroughwalls (Variables|flag|Getm_PassThroughWalls))
  (bind _returnvalue_3 (Math|Vector2D|MakeVector2D _returnvalue _returnvalue_2))
  (bind _returnvalue_4 (not _isaffectbyheight))
  (bind _returnvalue_5 (Math|Conversions|ToFloat(Integer) _mindistance))
  (bind _returnvalue_6 (Math|Conversions|ToFloat(Integer) _m_distances))
  (bind _playerheight (Variables|/Game/01_BP/03_Character/TopDownCharacter.TopDownCharacter_C|GetPlayerHeight _spellowner))
  (bind _returnvalue_7 (+ InVec _returnvalue_3))
  (bind _value (Utilities|Map|Find _struct_tiles _returnvalue_7))
  (bind (_x_2 _y_2) (Math|Vector2D|BreakVector2D _returnvalue_7))
  (bind _returnvalue_8 (!= (.unitonthistile _value) 0))
  (bind _can_walk_on_this_tile_valid (Default|CanJumponThisTiles grid (.height _value)))
  (bind _returnvalue_9 (< _playerheight (.height _value)))
  (bind _returnvalue_10 (- _x_2 _x))
  (bind _returnvalue_11 (- _y_2 _y))
  (bind _bsuccess (Utilities|Casting|CastToTopDownCharacter (.unitonthistile _value)))
  (bind _returnvalue_12 (Utilities|Enum|Equal(Enum) (.m_typesoftile _value) "NewEnumerator5"))
  (bind _returnvalue_13 (Utilities|Enum|Equal(Enum) (.m_typesoftile _value) "NewEnumerator6"))
  (bind _returnvalue_14 (not _bsuccess))
  (bind _returnvalue_15 (Math|Float|Absolute(Float) _returnvalue_10))
  (bind _returnvalue_16 (Math|Float|Absolute(Float) _returnvalue_11))
  (bind _returnvalue_17 (and _canattaquebellow _returnvalue_9))
  (bind _returnvalue_18 (Math|Boolean|ORBoolean _can_walk_on_this_tile_valid _returnvalue_4 _m_passthroughwalls))
  (bind _returnvalue_19 (Math|Boolean|ORBoolean _returnvalue_8 _returnvalue_13 _returnvalue_12 _returnvalue_14))
  (bind _returnvalue_20 (+ _returnvalue_15 _returnvalue_16))
  (bind _returnvalue_21 (or _returnvalue_17 _returnvalue_18))
  (bind _returnvalue_22 (> _returnvalue_20 _returnvalue_5))
  (bind _returnvalue_23 (<= _returnvalue_20 _returnvalue_6))
  (bind _returnvalue_24 (and _returnvalue_21 _returnvalue_19))
  (bind _returnvalue_25 (and _returnvalue_22 _returnvalue_23))
  (bind _returnvalue_26 (and _returnvalue_25 _returnvalue_24))
  (if _returnvalue_26
    (return _returnvalue_26 _returnvalue_7)))

(fn CheckForward
  (params (Array :type Array%20of%20Vector%202D%20Structures))
  (bind _spellowner (Variables|Default|GetSpellOwner))
  (bind _grid_index (Variables|/Game/01_BP/03_Character/TopDownCharacter.TopDownCharacter_C|Getgrid%20Index _spellowner))
  (bind (_x _y) (Math|Vector2D|BreakVector2D _grid_index))
  (for _array_element Array
    (if (or (== (.X (Math|Vector2D|BreakVector2D _array_element)) _x) (== (.Y (Math|Vector2D|BreakVector2D _array_element)) _y))
      (Utilities|Array|AddUnique (LocalVariables|GetReachableTaget) _array_element)))
  (return (LocalVariables|GetReachableTaget)))

(fn GetDamage
  (bind _currentmaxdamage (Variables|Value|GetCurrentMaxDamage))
  (bind _currentmindamage (Variables|Value|GetCurrentMinDamage))
  (bind _returnvalue (+ _currentmaxdamage 1))
  (bind _returnvalue_2 (Math|Random|RandomIntegerinRange _currentmindamage _returnvalue))
  (Development|PrintString (Utilities|String|ToString(Integer) _currentmindamage))
  (Development|PrintString (Utilities|String|ToString(Integer) _returnvalue_2))
  (return _returnvalue_2))

(fn GetHeightAction
  (params (height :type Integer))
  (bind _spellowner (Variables|Default|GetSpellOwner))
  (bind _playerheight (Variables|/Game/01_BP/03_Character/TopDownCharacter.TopDownCharacter_C|GetPlayerHeight _spellowner))
  (bind _returnvalue (- _playerheight height))
  (switch int _returnvalue
    (:Default
      (switch int (Math|Integer|Absolute(Integer) _returnvalue)
        (:Default
          (Variables|Value|SetCurrentMinDamage 0 :!label _label)
          (Variables|Value|SetCurrentMaxDamage 0))
        (:0
          (Variables|Value|SetCurrentMinDamage (Variables|Value|GetminDegats))
          (Variables|Value|SetCurrentMaxDamage (Variables|Value|GetmaxDegats)))
        (:1
          (Variables|Value|SetCurrentMinDamage (- (Variables|Value|GetminDegats) 1))
          (Variables|Value|SetCurrentMaxDamage (+ (Variables|Value|GetmaxDegats) 1)))
        (:2
          (goto _label))))
    (:0
      (Variables|Value|SetCurrentMinDamage (Variables|Value|GetminDegats))
      (Variables|Value|SetCurrentMaxDamage (Variables|Value|GetmaxDegats)))
    (:1
      (Variables|Value|SetCurrentMinDamage (+ (Variables|Value|GetminDegats) 1))
      (Variables|Value|SetCurrentMaxDamage (Variables|Value|GetmaxDegats)))
    (:2
      (Variables|Value|SetCurrentMinDamage (+ (Variables|Value|GetminDegats) 1))
      (Variables|Value|SetCurrentMaxDamage (- (Variables|Value|GetmaxDegats) 1)))))

(fn AffectDamage
  (params (targetUnit :type Top%20Down%20Character%20Object%20Reference) (height :type Integer))
  (CallFunction|GetHeightAction height)
  (Default|ETakeDamage targetUnit (CallFunction|GetDamage) (Variables|Default|GetSpellOwner))
  (Variables|Value|SetCurrentMinDamage (Variables|Value|GetminDegats))
  (Variables|Value|SetCurrentMaxDamage (Variables|Value|GetmaxDegats)))

(fn ManhattanDistance
  (params (Target :type Vector%202D%20Structure) (Position :type Vector%202D%20Structure))
  (bind (_x _y) (Math|Vector2D|BreakVector2D Target))
  (bind (_x_2 _y_2) (Math|Vector2D|BreakVector2D Position))
  (return (+ (Math|Float|Absolute(Float) (- _x_2 _x)) (Math|Float|Absolute(Float) (- _y_2 _y)))))

(fn IsATargetableUnit
  (params (Object :type Object%20Object%20Reference))
  (return (or (.bSuccess (Utilities|Casting|CastToTopDownCharacter Object)) (.bSuccess (Utilities|Casting|CastToBP_Fiente Object)))))

(fn CanAccestoThisTIlewithRayCast
  (params (TargetableTile :type Array%20of%20Vector%202D%20Structures) (gridManager :type Grid%20Behaviours%20Object%20Reference))
  (LocalVariables|SetGrid gridManager)
  (Utilities|IsValid (Variables|Default|GetSpellOwner)
    (:Is%20Valid
      (for _array_element TargetableTile
        (bind _returnvalue (Collision|LineTraceByChannel (Transformation|GetWorldLocation (Variables|/Game/01_BP/03_Character/TopDownCharacter.TopDownCharacter_C|GetStartRay (Variables|Default|GetSpellOwner))) (.m_tiles_worldlocation (.Value (Utilities|Map|Find (Variables|/Game/01_BP/Grid/GridBehaviours.GridBehaviours_C|Getstruct_Tiles (LocalVariables|GetGrid)) _array_element))) "TraceTypeQuery4" false 0 "ForDuration"))
        (if _returnvalue
          (Utilities|Array|AddUnique (LocalVariables|GetCantAcces) (.m_tiles_index (.Value (Utilities|Map|Find (Variables|/Game/01_BP/Grid/GridBehaviours.GridBehaviours_C|Getstruct_Tiles (LocalVariables|GetGrid)) _array_element))))))
      (return (LocalVariables|GetCantAcces)))))

(fn AddUntargatableTiles
  (params (gridManager :type Grid%20Behaviours%20Object%20Reference) (TargetableTile :type Array%20of%20Vector%202D%20Structures))
  (bind _cantacces1 (CallFunction|CanAccestoThisTIlewithRayCast TargetableTile gridManager))
  (for _array_element _cantacces1
    (if (not (Utilities|Array|ContainsItem (Variables|Liste|GetUnAttackableTiles) _array_element))
      (if (not (Variables|flag|Getm_PassThroughWalls))
        (Utilities|Array|AddUnique (Variables|Liste|GetUnAttackableTiles) _array_element)))))