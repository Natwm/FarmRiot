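; Ultimate spell for the Rushdown rabbit characters on the tactical grid, spending all the caster's points on one attack.
; Targeting highlights tiles in range, splitting off unreachable ones as unattackable unless the spell passes through walls.
; Character damage scales by 10% per point before points are zeroed, while BP_Fiente targets take unscaled max damage.
; Montage and spell icon follow the brown or black rabbit variant; montage completion deselects the spell.
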(event EventBeginPlay
  (|CallParentFunction) ; This node is disabled and will not be called.\nDrag off pins to build functionality.
)

(event EventEShowTilesTargetedbySpell
  (params (Origin%20Index :type Vector%202D%20Structure) (Grid :type Grid%20Behaviours%20Object%20Reference) (Show%20Tiles :type Boolean))
  (Variables|Default|SetCurrentPointCost (Variables|/Game/01_BP/03_Character/TopDownCharacter.TopDownCharacter_C|GetNbPoint (Variables|Default|GetSpellOwner)))
  (if (> (Utilities|Array|Length (Variables|Default|GetReachableTarget)) 0)
    (Default|HighlightAttackableTiles Grid (Variables|Default|GetReachableTarget) false)
    (Utilities|Array|Clear (Variables|Default|GetAttackableTiles))
    (Utilities|Array|Clear (Variables|Default|GetUnAttackableTiles))
    (Utilities|Array|Clear (Variables|Default|GetReachableTarget)))
  (bind _newlocalvar_01 (CallFunction|GetAttackableTiles Origin%20Index Grid))
  (bind _reachablestargets (CallFunction|GetReachableTargetatMinimumDistances _newlocalvar_01 Origin%20Index))
  (Variables|Default|SetReachableTarget _reachablestargets)
  (bind _reachable_tiles (Default|GetPossibleTargetIndex Grid (Variables|/Game/01_BP/03_Character/TopDownCharacter.TopDownCharacter_C|Getgrid%20Index (Variables|Default|GetSpellOwner)) (Variables|Default|GetcurrentDistance)))
  (if (not (Variables|Default|Getm_PassThroughWalls))
    (for _array_element (Variables|Default|GetReachableTarget)
      (if (Utilities|Array|ContainsItem _reachable_tiles _array_element)
        (Utilities|Array|AddUnique (Variables|Default|GetAttackableTiles) _array_element)
        (else
          (Utilities|Array|AddUnique (Variables|Default|GetUnAttackableTiles) _array_element)
          (Utilities|Array|RemoveItem (Variables|Default|GetAttackableTiles) _array_element)
          (Utilities|Array|RemoveItem (Variables|Default|GetReachableTarget) _array_element))))
    (else
      (Variables|Default|SetAttackableTiles (Variables|Default|GetReachableTarget))))
  (Default|HighlightAttackableTiles Grid (Variables|Default|GetAttackableTiles) Show%20Tiles)
  (if (not (Variables|Default|Getm_PassThroughWalls))
    (CallFunction|AddUntargatableTiles Grid (Variables|Default|GetReachableTarget))
    (Default|HighlighUnAttackableTiles Grid (Variables|Default|GetUnAttackableTiles) Show%20Tiles)))

(event EventEUseSpellonTarget
  (params (Grid :type Grid%20Behaviours%20Object%20Reference) (Target%20position :type Vector%202D%20Structure) (SpellOwner :type Top%20Down%20Character%20Object%20Reference))
  (bind _struct_tiles (Variables|/Game/01_BP/Grid/GridBehaviours.GridBehaviours_C|Getstruct_Tiles Grid))
  (bind _value (Utilities|Map|Find _struct_tiles Target%20position))
  (if (and (Utilities|Array|ContainsItem (Variables|Default|GetAttackableTiles) Target%20position) (not (Utilities|Array|ContainsItem (Variables|Default|GetUnAttackableTiles) Target%20position)))
    (if (Math|Boolean|ANDBoolean (CallFunction|IsATargetableUnit (.unitonthistile _value)) (Utilities|Enum|NotEqual(Enum) (.m_typesoftile _value) "NewEnumerator5") (Utilities|Enum|NotEqual(Enum) (.m_typesoftile _value) "NewEnumerator6"))
      (bind _astop_down_character (Utilities|Casting|CastToTopDownCharacter (.unitonthistile _value))
        (:then
          (CallFunction|AffectDamage _astop_down_character (.height _value)))
        (:CastFailed
          (bind _asbp_fiente (Utilities|Casting|CastToBP_Fiente (.unitonthistile _value)))
          (Default|ETakeDamage _asbp_fiente (Variables|Default|GetmaxDegats))))
      (CallFunction|ReduceInit)
      (bind (_targetmesh _animmotagetouse1) (CallFunction|PlaySpellAnimation))
      (Animation|Montage|PlayMontage (Variables|/Script/Engine.Character|GetMesh _targetmesh) _animmotagetouse1
        (:OnCompleted
          (Variables|Default|SetcurrentDistance (Variables|Default|Getm_Distances))
          (Class|FMODAudioComponent|Play (Variables|Default|GetAttaque_FMODAudio))
          (Default|CallEDShowInformation _astop_down_character _astop_down_character)
          (Default|EDeselectSpeel SpellOwner)))
      (else
        (Class|FMODAudioComponent|Play (Variables|Default|GetCantAttaque_FMODAudio) :!label _label)))
    (else
      (goto _label))))

(fn ConstructionScript
  (|CallParentFunction))

(fn ReduceInit
  (params (Direction :type Vector%202D%20Structure))
  (Variables|/Game/01_BP/03_Character/TopDownCharacter.TopDownCharacter_C|SetNbPoint (Variables|Default|GetSpellOwner) 0))

(fn AffectDamage
  (params (targetUnit :type Top%20Down%20Character%20Object%20Reference) (height :type Integer))
  (CallFunction|UseAllPoint)
  (|CallParentFunction targetUnit height))

(fn UseAllPoint
  (bind _spellowner (Variables|Default|GetSpellOwner))
  (bind _nbpoint (Variables|/Game/01_BP/03_Character/TopDownCharacter.TopDownCharacter_C|GetNbPoint _spellowner))
  (bind _returnvalue (Math|Conversions|ToFloat(Integer) _nbpoint))
  (bind _returnvalue_2 (/ _returnvalue 1e+01))
  (bind _returnvalue_3 (+ 1.0 _returnvalue_2))
  (Variables|Default|SetCurrentMaxDamage (Math|Float|Round (* (Variables|Default|GetCurrentMaxDamage) _returnvalue_3)))
  (Variables|Default|SetCurrentMinDamage (Math|Float|Round (* (Variables|Default|GetCurrentMinDamage) _returnvalue_3))))

(fn PlaySpellAnimation
  (bind _asrushdown_character_rabbit_brown (Utilities|Casting|CastToRushdown_Character_Rabbit_Brown (Variables|Default|GetSpellOwner))
    (:then
      (LocalVariables|SetTarget _asrushdown_character_rabbit_brown)
      (LocalVariables|SetAnimToUSe "/Game/06_Animation/Anim_Brown/Rabbit/RabbitBrown_Ultime_AM.RabbitBrown_Ultime_AM"))
    (:CastFailed
      (bind _asrushdown_character_rabit_black (Utilities|Casting|CastToRushdown_Character_Rabit_Black (Variables|Default|GetSpellOwner)))
      (LocalVariables|SetTarget _asrushdown_character_rabit_black)
      (LocalVariables|SetAnimToUSe "/Game/06_Animation/Anim_Dark/Rabbit/RabbitDark_Ultime_AM.RabbitDark_Ultime_AM")))
  (return (LocalVariables|GetTarget) (LocalVariables|GetAnimToUSe)))

(fn GetImagetoDisplay
  (bind _spellowner (Variables|Default|GetSpellOwner))
  (Utilities|Casting|CastToRushdown_Character_Rabit_Black _spellowner
    (:then
      (LocalVariables|SetTexture%20to%20display "/Game/07_UI/Interfqce/interface_sort/Lapin/lapin_NOIR_-_sort_3.lapin_NOIR_-_sort_3"))
    (:CastFailed
      (Utilities|Casting|CastToRushdown_Character_Rabbit_Brown _spellowner)
      (LocalVariables|SetTexture%20to%20display "/Game/07_UI/Interfqce/interface_sort/Lapin/lapin_MARRON_-_sort_3.lapin_MARRON_-_sort_3")))
  (return (LocalVariables|GetTexture%20to%20display)))