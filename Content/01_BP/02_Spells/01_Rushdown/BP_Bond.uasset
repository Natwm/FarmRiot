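; Bond is the Rushdown rabbits' leap spell, moving the caster to a reachable grid tile with per-rabbit montage and icon.
; Drops of one or two height levels trigger an impact before landing, with two also damaging adjacent characters.
; PushByJump handles only the first neighbour, and an invalid push tile cancels the leap.
; Push applies damage, fall effects or a debuff depending on height and what blocks the destination.
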(event EventEUseSpellonTarget
  (params (Grid :type Grid%20Behaviours%20Object%20Reference) (Target%20position :type Vector%202D%20Structure) (SpellOwner :type Top%20Down%20Character%20Object%20Reference))
  (bind (_x _y) (Math|Vector2D|BreakVector2D Target%20position))
  (bind _struct_tiles (Variables|/Game/01_BP/Grid/GridBehaviours.GridBehaviours_C|Getstruct_Tiles Grid))
  (bind _value (Utilities|Map|Find _struct_tiles Target%20position))
  (if (and (> _x 0.0) (> _y 0.0))
    (if (and (Utilities|Array|ContainsItem (Variables|Default|GetReachableTarget) Target%20position) true)
      (if (Math|Boolean|ANDBoolean (not (.bSuccess (Utilities|Casting|CastToTopDownCharacter (.unitonthistile _value)))) (Utilities|Enum|NotEqual(Enum) (.m_typesoftile _value) "NewEnumerator5") (Utilities|Enum|NotEqual(Enum) (.m_typesoftile _value) "NewEnumerator6"))
        (switch int (- (Variables|/Game/01_BP/03_Character/TopDownCharacter.TopDownCharacter_C|GetPlayerHeight (Variables|Default|GetSpellOwner)) (.height _value))
          (:Default
            (Transformation|SetActorLocation (Variables|Default|GetSpellOwner) (.m_tiles_worldlocation _value) false true :!label _label)
            (Variables|/Game/01_BP/03_Character/TopDownCharacter.TopDownCharacter_C|SetPlayerHeight (Variables|Default|GetSpellOwner) (.height _value))
            (Default|GetUnitonTile (Variables|Default|GetSpellOwner) Target%20position)
            (CallFunction|ReduceInit)
            (bind (_targetmesh _animmotagetouse1) (CallFunction|PlaySpellAnimation))
            (Animation|Montage|PlayMontage (Variables|/Script/Engine.Character|GetMesh _targetmesh) _animmotagetouse1
              (:OnCompleted
                (Default|EDeselectSpeel (Variables|Default|GetSpellOwner))
                (Class|FMODAudioComponent|Play (Variables|Default|GetAttaque_FMODAudio)))))
          (:0
            (goto _label))
          (:1
            (Variables|Flag|SetUseSpecial false)
            (bind _returnvalue (CallFunction|SpecialJumpAction Grid Target%20position :!label _label_2))
            (if _returnvalue
              (goto _label)
              (else
                (Class|FMODAudioComponent|Play (Variables|Default|GetCantAttaque_FMODAudio) :!label _label_3))))
          (:2
            (Variables|Flag|SetUseSpecial true)
            (goto _label_2)))
        (else
          (goto _label_3))))))

(fn ConstructionScript
  (|CallParentFunction))

(fn GetTilesArroundforEffects
  (params (Grid :type Grid%20Behaviours%20Object%20Reference) (TargetIndex :type Vector%202D%20Structure))
  (bind _output_get (LocalVariables|SetGridManager Grid))
  (bind _reachable_tiles (Default|GetPossibleTargetIndexinStraightLines _output_get TargetIndex 1))
  (for _array_element _reachable_tiles
    (if (!= (.unitonthistile (.Value (Utilities|Map|Find (Variables|/Game/01_BP/Grid/GridBehaviours.GridBehaviours_C|Getstruct_Tiles (LocalVariables|GetGridManager)) _array_element))) 0)
      (Utilities|Casting|CastToTopDownCharacter (.unitonthistile (.Value (Utilities|Map|Find (Variables|/Game/01_BP/Grid/GridBehaviours.GridBehaviours_C|Getstruct_Tiles (LocalVariables|GetGridManager)) _array_element)))
        (:then
          _)
        (:CastFailed
          (Utilities|Casting|CastToBP_MovableObstacle (.unitonthistile (.Value (Utilities|Map|Find (Variables|/Game/01_BP/Grid/GridBehaviours.GridBehaviours_C|Getstruct_Tiles (LocalVariables|GetGridManager)) _array_element))))))
      (Utilities|Array|AddUnique (LocalVariables|GetTargetableUnit) _array_element)))
  (return (LocalVariables|GetTargetableUnit)))

(fn DamageUnitbyPropultion
  (params (Tagets :type Array%20of%20Vector%202D%20Structures) (Grid%20Manager :type Grid%20Behaviours%20Object%20Reference))
  (LocalVariables|SetGridManager Grid%20Manager)
  (for _array_element Tagets
    (if (Math|Vector|NotEqual(Vector) _array_element (Variables|/Game/01_BP/03_Character/TopDownCharacter.TopDownCharacter_C|Getgrid%20Index (Variables|Default|GetSpellOwner)) 0.0001)
      (bind _astop_down_character (Utilities|Casting|CastToTopDownCharacter (.unitonthistile (.Value (Utilities|Map|Find (Variables|/Game/01_BP/Grid/GridBehaviours.GridBehaviours_C|Getstruct_Tiles (LocalVariables|GetGridManager)) _array_element)))))
      (if (!= _astop_down_character (Variables|Default|GetSpellOwner))
        (Default|ETakeDamage _astop_down_character (Variables|Default|GetmaxDegats))))))

(fn PushbyJump
  (params (GridManager :type Grid%20Behaviours%20Object%20Reference) (Targets :type Array%20of%20Vector%202D%20Structures) (JumpPosition :type Vector%202D%20Structure))
  (LocalVariables|SetGrid GridManager)
  (if (> (Utilities|Array|Length Targets) 0)
    (for _array_element Targets
      (bind _astop_down_character (Utilities|Casting|CastToTopDownCharacter (.unitonthistile (.Value (Utilities|Map|Find (Variables|/Game/01_BP/Grid/GridBehaviours.GridBehaviours_C|Getstruct_Tiles (LocalVariables|GetGrid)) _array_element)))))
      (if (Math|Boolean|ANDBoolean (> (.X (Math|Vector2D|BreakVector2D (CallFunction|GetDirection (Variables|/Game/01_BP/03_Character/TopDownCharacter.TopDownCharacter_C|Getgrid%20Index _astop_down_character) JumpPosition))) 0.0) (> (.Y (Math|Vector2D|BreakVector2D (CallFunction|GetDirection (Variables|/Game/01_BP/03_Character/TopDownCharacter.TopDownCharacter_C|Getgrid%20Index _astop_down_character) JumpPosition))) 0.0) (Utilities|Enum|NotEqual(Enum) (.m_typesoftile (.Value (Utilities|Map|Find (Variables|/Game/01_BP/Grid/GridBehaviours.GridBehaviours_C|Getstruct_Tiles (LocalVariables|GetGrid)) (CallFunction|GetDirection (Variables|/Game/01_BP/03_Character/TopDownCharacter.TopDownCharacter_C|Getgrid%20Index _astop_down_character) JumpPosition)))) "NewEnumerator5") (Utilities|Enum|NotEqual(Enum) (.m_typesoftile (.Value (Utilities|Map|Find (Variables|/Game/01_BP/Grid/GridBehaviours.GridBehaviours_C|Getstruct_Tiles (LocalVariables|GetGrid)) (CallFunction|GetDirection (Variables|/Game/01_BP/03_Character/TopDownCharacter.TopDownCharacter_C|Getgrid%20Index _astop_down_character) JumpPosition)))) "NewEnumerator6"))
        (CallFunction|Push _astop_down_character JumpPosition (LocalVariables|GetGrid)))
      (return (Math|Boolean|ANDBoolean (> (.X (Math|Vector2D|BreakVector2D (CallFunction|GetDirection (Variables|/Game/01_BP/03_Character/TopDownCharacter.TopDownCharacter_C|Getgrid%20Index _astop_down_character) JumpPosition))) 0.0) (> (.Y (Math|Vector2D|BreakVector2D (CallFunction|GetDirection (Variables|/Game/01_BP/03_Character/TopDownCharacter.TopDownCharacter_C|Getgrid%20Index _astop_down_character) JumpPosition))) 0.0) (Utilities|Enum|NotEqual(Enum) (.m_typesoftile (.Value (Utilities|Map|Find (Variables|/Game/01_BP/Grid/GridBehaviours.GridBehaviours_C|Getstruct_Tiles (LocalVariables|GetGrid)) (CallFunction|GetDirection (Variables|/Game/01_BP/03_Character/TopDownCharacter.TopDownCharacter_C|Getgrid%20Index _astop_down_character) JumpPosition)))) "NewEnumerator5") (Utilities|Enum|NotEqual(Enum) (.m_typesoftile (.Value (Utilities|Map|Find (Variables|/Game/01_BP/Grid/GridBehaviours.GridBehaviours_C|Getstruct_Tiles (LocalVariables|GetGrid)) (CallFunction|GetDirection (Variables|/Game/01_BP/03_Character/TopDownCharacter.TopDownCharacter_C|Getgrid%20Index _astop_down_character) JumpPosition)))) "NewEnumerator6"))))
    (else
      (return true))))

(fn Push
  (params (SpellTargetPosition :type Top%20Down%20Character%20Object%20Reference) (FuturSpellOwnerPosition :type Vector%202D%20Structure) (GridManager :type Grid%20Behaviours%20Object%20Reference))
  (LocalVariables|SetTarget SpellTargetPosition)
  (LocalVariables|SetCaster FuturSpellOwnerPosition)
  (LocalVariables|SetGrid GridManager)
  (if (== (.unitonthistile (.Value (Utilities|Map|Find (Variables|/Game/01_BP/Grid/GridBehaviours.GridBehaviours_C|Getstruct_Tiles (LocalVariables|GetGrid)) (CallFunction|GetDirection (Variables|/Game/01_BP/03_Character/TopDownCharacter.TopDownCharacter_C|Getgrid%20Index (LocalVariables|GetTarget)) (LocalVariables|GetCaster))))) 0)
    (if (>= (- (Variables|/Game/01_BP/03_Character/TopDownCharacter.TopDownCharacter_C|GetPlayerHeight (LocalVariables|GetTarget)) (.height (.Value (Utilities|Map|Find (Variables|/Game/01_BP/Grid/GridBehaviours.GridBehaviours_C|Getstruct_Tiles (LocalVariables|GetGrid)) (CallFunction|GetDirection (Variables|/Game/01_BP/03_Character/TopDownCharacter.TopDownCharacter_C|Getgrid%20Index (LocalVariables|GetTarget)) (LocalVariables|GetCaster)))))) 0)
      (switch int (- (Variables|/Game/01_BP/03_Character/TopDownCharacter.TopDownCharacter_C|GetPlayerHeight (LocalVariables|GetTarget)) (.height (.Value (Utilities|Map|Find (Variables|/Game/01_BP/Grid/GridBehaviours.GridBehaviours_C|Getstruct_Tiles (LocalVariables|GetGrid)) (CallFunction|GetDirection (Variables|/Game/01_BP/03_Character/TopDownCharacter.TopDownCharacter_C|Getgrid%20Index (LocalVariables|GetTarget)) (LocalVariables|GetCaster))))))
        (:0
          _)
        (:1
          (Default|ETakeDamage (LocalVariables|GetTarget) (/ (Variables|Default|GetmaxDegats) 2)))
        (:2
          (Default|ETakeDamage (LocalVariables|GetTarget) (Variables|Default|GetmaxDegats))
          (CallFunction|FallEffect (LocalVariables|GetTarget) (.height (.Value (Utilities|Map|Find (Variables|/Game/01_BP/Grid/GridBehaviours.GridBehaviours_C|Getstruct_Tiles (LocalVariables|GetGrid)) (CallFunction|GetDirection (Variables|/Game/01_BP/03_Character/TopDownCharacter.TopDownCharacter_C|Getgrid%20Index (LocalVariables|GetTarget)) (LocalVariables|GetCaster))))))))
      (Transformation|SetActorLocation (LocalVariables|GetTarget) (.m_tiles_worldlocation (.Value (Utilities|Map|Find (Variables|/Game/01_BP/Grid/GridBehaviours.GridBehaviours_C|Getstruct_Tiles (LocalVariables|GetGrid)) (CallFunction|GetDirection (Variables|/Game/01_BP/03_Character/TopDownCharacter.TopDownCharacter_C|Getgrid%20Index (LocalVariables|GetTarget)) (LocalVariables|GetCaster))))) false false)
      (Default|GetUnitonTile (LocalVariables|GetTarget))
      (Default|ETakeDamage (LocalVariables|GetTarget) (Variables|Default|GetmaxDegats))
      (else
        (Default|ETakeDamage (LocalVariables|GetTarget) (/ (Variables|Default|GetmaxDegats) 2))))
    (elif (.bSuccess (Utilities|Casting|CastToTopDownCharacter (.unitonthistile (.Value (Utilities|Map|Find (Variables|/Game/01_BP/Grid/GridBehaviours.GridBehaviours_C|Getstruct_Tiles (LocalVariables|GetGrid)) (CallFunction|GetDirection (Variables|/Game/01_BP/03_Character/TopDownCharacter.TopDownCharacter_C|Getgrid%20Index (LocalVariables|GetTarget)) (LocalVariables|GetCaster)))))))
      (Default|ETakeDamage (.AsTop%20Down%20Character (Utilities|Casting|CastToTopDownCharacter (.unitonthistile (.Value (Utilities|Map|Find (Variables|/Game/01_BP/Grid/GridBehaviours.GridBehaviours_C|Getstruct_Tiles (LocalVariables|GetGrid)) (CallFunction|GetDirection (Variables|/Game/01_BP/03_Character/TopDownCharacter.TopDownCharacter_C|Getgrid%20Index (LocalVariables|GetTarget)) (LocalVariables|GetCaster))))))) (/ (Variables|Default|GetmaxDegats) 2))
      (else
        ;[1 1 1] Apply a debuf on the speed
        (if (.bSuccess (Utilities|Casting|CastToBP_Base_Obstacle (.unitonthistile (.Value (Utilities|Map|Find (Variables|/Game/01_BP/Grid/GridBehaviours.GridBehaviours_C|Getstruct_Tiles (LocalVariables|GetGrid)) (CallFunction|GetDirection (Variables|/Game/01_BP/03_Character/TopDownCharacter.TopDownCharacter_C|Getgrid%20Index (LocalVariables|GetTarget)) (LocalVariables|GetCaster)))))))
          (Default|EApplyDebuff (LocalVariables|GetTarget) (Variables|Default|GetInitDebuffValue) (Variables|Default|GetDebuffTime)))))))

(fn SpecialJumpAction
  (params (grid :type Grid%20Behaviours%20Object%20Reference) (targetIndex :type Vector%202D%20Structure))
  (LocalVariables|Setmanager grid)
  (if (Variables|Flag|GetUseSpecial)
    (CallFunction|DamageUnitbyPropultion (CallFunction|GetTilesArroundforEffects (LocalVariables|Getmanager) targetIndex) (LocalVariables|Getmanager)))
  (bind _returnvalue (CallFunction|PushbyJump (LocalVariables|Getmanager) (CallFunction|GetTilesArroundforEffects (LocalVariables|Getmanager) targetIndex) targetIndex))
  (return _returnvalue))

(fn PlaySpellAnimation
  (bind _asrushdown_character_rabbit_brown (Utilities|Casting|CastToRushdown_Character_Rabbit_Brown (Variables|Default|GetSpellOwner))
    (:then
      (LocalVariables|SetTarget _asrushdown_character_rabbit_brown)
      (LocalVariables|SetAnimToUSe "/Game/06_Animation/Anim_Brown/Rabbit/RabbitBrown_Bond_AM.RabbitBrown_Bond_AM"))
    (:CastFailed
      (bind _asrushdown_character_rabit_black (Utilities|Casting|CastToRushdown_Character_Rabit_Black (Variables|Default|GetSpellOwner)))
      (LocalVariables|SetTarget _asrushdown_character_rabit_black)
      (LocalVariables|SetAnimToUSe "/Game/06_Animation/Anim_Dark/Rabbit/RabbitDark_Bond_AM.RabbitDark_Bond_AM")))
  (return (LocalVariables|GetTarget) (LocalVariables|GetAnimToUSe)))

(fn GetImagetoDisplay
  (bind _spellowner (Variables|Default|GetSpellOwner))
  (Utilities|Casting|CastToRushdown_Character_Rabit_Black _spellowner
    (:then
      (LocalVariables|SetTexture%20to%20display "/Game/07_UI/Interfqce/interface_sort/Lapin/lapin_NOIR_-_sort_2.lapin_NOIR_-_sort_2"))
    (:CastFailed
      (Utilities|Casting|CastToRushdown_Character_Rabbit_Brown _spellowner)
      (LocalVariables|SetTexture%20to%20display "/Game/07_UI/Interfqce/interface_sort/Lapin/lapin_MARRON_-_sort_2.lapin_MARRON_-_sort_2")))
  (return (LocalVariables|GetTexture%20to%20display)))