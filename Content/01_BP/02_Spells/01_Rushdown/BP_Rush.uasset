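; Rush spell for the grid tactics game: highlights straight-line targets, then teleports the caster along the chosen direction, with range increased at height 2.
; NewFunction00 builds the path, extending past occupied end tiles to a free one.
; EUseSpellonTarget blocks two tile types as landings and deals damage once per unit on the path, but always to the landing tile's occupant.
; RushActionResult and RushActionApply are unused by the live flow.
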(event EventEUseSpellonTarget
  (params (Grid :type Grid%20Behaviours%20Object%20Reference) (Target%20position :type Vector%202D%20Structure) (SpellOwner :type Top%20Down%20Character%20Object%20Reference))
  (Variables|Default|SetCheckPosition (Variables|/Game/01_BP/03_Character/TopDownCharacter.TopDownCharacter_C|Getgrid%20Index (Variables|Default|GetSpellOwner)))
  (bind _affectedtile (CallFunction|NewFunction00 Grid Target%20position SpellOwner))
  (bind _array_element (Utilities|Array|ForEachLoopwithBreak _affectedtile :!label _label)
    (:LoopBody
      (Utilities|Casting|CastToTopDownCharacter (.unitonthistile (.Value (Utilities|Map|Find (Variables|/Game/01_BP/Grid/GridBehaviours.GridBehaviours_C|Getstruct_Tiles Grid) _array_element)))
        (:then
          (Utilities|Array|Add (Variables|Default|GetAttackableTiles) (.m_tiles_index (.Value (Utilities|Map|Find (Variables|/Game/01_BP/Grid/GridBehaviours.GridBehaviours_C|Getstruct_Tiles Grid) _array_element)))))
        (:CastFailed
          _))
      (if (< (CallFunction|ManhattanDistance (Variables|Default|GetCheckPosition) _array_element) 0.0)
        (if (or (Utilities|Enum|NotEqual(Enum) (.m_typesoftile (.Value (Utilities|Map|Find (Variables|/Game/01_BP/Grid/GridBehaviours.GridBehaviours_C|Getstruct_Tiles Grid) _array_element))) "NewEnumerator5") (Utilities|Enum|NotEqual(Enum) (.m_typesoftile (.Value (Utilities|Map|Find (Variables|/Game/01_BP/Grid/GridBehaviours.GridBehaviours_C|Getstruct_Tiles Grid) _array_element))) "NewEnumerator6"))
          (Variables|Default|SetCheckPosition (.m_tiles_index (.Value (Utilities|Map|Find (Variables|/Game/01_BP/Grid/GridBehaviours.GridBehaviours_C|Getstruct_Tiles Grid) _array_element))))
          (else
            (goto _label Break)))))
    (:Completed
      (Variables|Default|SetCheckPosition (Utilities|Array|Get(acopy) _affectedtile (Utilities|Array|LastIndex _affectedtile)))
      (if (and (Utilities|Enum|NotEqual(Enum) (.m_typesoftile (.Value (Utilities|Map|Find (Variables|/Game/01_BP/Grid/GridBehaviours.GridBehaviours_C|Getstruct_Tiles Grid) (Variables|Default|GetCheckPosition)))) "NewEnumerator5") (Utilities|Enum|NotEqual(Enum) (.m_typesoftile (.Value (Utilities|Map|Find (Variables|/Game/01_BP/Grid/GridBehaviours.GridBehaviours_C|Getstruct_Tiles Grid) (Variables|Default|GetCheckPosition)))) "NewEnumerator6"))
        (Transformation|SetActorLocation (Variables|Default|GetSpellOwner) (.m_tiles_worldlocation (.Value (Utilities|Map|Find (Variables|/Game/01_BP/Grid/GridBehaviours.GridBehaviours_C|Getstruct_Tiles Grid) (Variables|Default|GetCheckPosition)))) false false)
        (Default|GetUnitonTile (Variables|Default|GetSpellOwner) (.m_tiles_index (.Value (Utilities|Map|Find (Variables|/Game/01_BP/Grid/GridBehaviours.GridBehaviours_C|Getstruct_Tiles Grid) (Variables|Default|GetCheckPosition)))))
        (for _array_element_2 (Variables|Default|GetAttackableTiles)
          (bind _astop_down_character (Utilities|Casting|CastToTopDownCharacter (.unitonthistile (.Value (Utilities|Map|Find (Variables|/Game/01_BP/Grid/GridBehaviours.GridBehaviours_C|Getstruct_Tiles Grid) (Variables|Default|GetCheckPosition))))))
          (Default|ETakeDamage _astop_down_character (CallFunction|GetDamage)))
        (Default|EDeselectSpeel (Variables|Default|GetSpellOwner))
        (CallFunction|ReduceInit)
        (Class|FMODAudioComponent|Play (Variables|Default|GetAttaque_FMODAudio))
        (else
          (Class|FMODAudioComponent|Play (Variables|Default|GetCantAttaque_FMODAudio)))))))

(event EventEShowTilesTargetedbySpell
  (params (Origin%20Index :type Vector%202D%20Structure) (Grid :type Grid%20Behaviours%20Object%20Reference) (Show%20Tiles :type Boolean))
  (if (== (Variables|/Game/01_BP/03_Character/TopDownCharacter.TopDownCharacter_C|GetPlayerHeight (Variables|Default|GetSpellOwner)) 2)
    (Math|Integer|IncrementInt (Variables|Default|Getm_Distances)
      (:%20%20
        (Math|Integer|IncrementInt (Variables|Default|GetMinDistance)
          (:%20%20
            _)))))
  (if (> (Utilities|Array|Length (Variables|Default|GetReachableTarget)) 0)
    (Default|HighlightAttackableTiles Grid (Variables|Default|GetReachableTarget) false)
    (Utilities|Array|Clear (Variables|Default|GetReachableTarget)))
  (bind _newlocalvar_01 (CallFunction|GetAttackableTiles Origin%20Index Grid))
  (bind _reachablestargets (CallFunction|GetReachableTargetatMinimumDistances _newlocalvar_01 Origin%20Index))
  (if (Variables|Flag|GetIsStraightLineq)
    (bind _reachabletiles (CallFunction|CheckForward _reachablestargets))
    (bind _output_get (Variables|Default|SetReachableTarget _reachabletiles))
    (CallFunction|AddUntargatableTiles Grid _output_get)
    (Default|HighlightAttackableTiles Grid (Variables|Default|GetReachableTarget) Show%20Tiles)
    (Default|HighlighUnAttackableTiles Grid (Variables|Default|GetUnAttackableTiles) Show%20Tiles)))

(fn ConstructionScript
  (|CallParentFunction))

(fn RushActionResult
  (params (Grid :type Grid%20Behaviours%20Object%20Reference) (target :type Vector%202D%20Structure))
  (LocalVariables|SetLocatTargetTile target)
  (LocalVariables|SetDirection (Math|Vector2D|Normalize2D (- (Variables|/Game/01_BP/03_Character/TopDownCharacter.TopDownCharacter_C|Getgrid%20Index (Variables|Default|GetSpellOwner)) target)))
  (for _index (range (Variables|Default|Getm_Distances) (Variables|Default|Getm_Distances))
    (LocalVariables|SetLocatTargetTile (- (Variables|/Game/01_BP/03_Character/TopDownCharacter.TopDownCharacter_C|Getgrid%20Index (Variables|Default|GetSpellOwner)) (LocalVariables|GetDirection)))
    (if (.bSuccess (Utilities|Casting|CastToTopDownCharacter (.unitonthistile (.Value (Utilities|Map|Find (Variables|/Game/01_BP/Grid/GridBehaviours.GridBehaviours_C|Getstruct_Tiles Grid) (LocalVariables|GetLocatTargetTile))))))
      (Utilities|Array|AddUnique (LocalVariables|GetAffectedTiles) (LocalVariables|GetLocatTargetTile))))
  (while (.bSuccess (Utilities|Casting|CastToTopDownCharacter (.unitonthistile (.Value (Utilities|Map|Find (Variables|/Game/01_BP/Grid/GridBehaviours.GridBehaviours_C|Getstruct_Tiles Grid) (LocalVariables|GetLocatTargetTile))))))
    (Utilities|Array|AddUnique (LocalVariables|GetAffectedTiles) (LocalVariables|GetLocatTargetTile))
    (LocalVariables|SetLocatTargetTile (- (LocalVariables|GetLocatTargetTile) (LocalVariables|GetDirection)))
    (if (not (.bSuccess (Utilities|Casting|CastToTopDownCharacter (.unitonthistile (.Value (Utilities|Map|Find (Variables|/Game/01_BP/Grid/GridBehaviours.GridBehaviours_C|Getstruct_Tiles Grid) (LocalVariables|GetLocatTargetTile)))))))
      (if (Math|Boolean|ANDBoolean (== (.unitonthistile (.Value (Utilities|Map|Find (Variables|/Game/01_BP/Grid/GridBehaviours.GridBehaviours_C|Getstruct_Tiles Grid) (LocalVariables|GetLocatTargetTile)))) 0) (Utilities|Enum|NotEqual(Enum) (.m_typesoftile (.Value (Utilities|Map|Find (Variables|/Game/01_BP/Grid/GridBehaviours.GridBehaviours_C|Getstruct_Tiles Grid) (LocalVariables|GetLocatTargetTile)))) "NewEnumerator6") (Utilities|Enum|NotEqual(Enum) (.m_typesoftile (.Value (Utilities|Map|Find (Variables|/Game/01_BP/Grid/GridBehaviours.GridBehaviours_C|Getstruct_Tiles Grid) (LocalVariables|GetLocatTargetTile)))) "NewEnumerator5"))
        (Utilities|Array|AddUnique (LocalVariables|GetAffectedTiles) (LocalVariables|GetLocatTargetTile))
        (return (LocalVariables|GetAffectedTiles))))))

(fn RushActionApply
  (params (Grid :type Grid%20Behaviours%20Object%20Reference) (target :type Vector%202D%20Structure))
  (bind _struct_tiles (Variables|/Game/01_BP/Grid/GridBehaviours.GridBehaviours_C|Getstruct_Tiles Grid))
  (bind _value (Utilities|Map|Find _struct_tiles target))
  (bind (_astop_down_character _bsuccess) (Utilities|Casting|CastToTopDownCharacter (.unitonthistile _value)))
  (if _bsuccess
    (Default|ETakeDamage _astop_down_character (Variables|Default|GetmaxDegats))))

(fn NewFunction00
  (params (grid :type Grid%20Behaviours%20Object%20Reference%20%28by%20ref%29) (pos :type Vector%202D%20Structure) (target :type Top%20Down%20Character%20Object%20Reference))
  (LocalVariables|SetGridManager grid)
  (bind _output_get (LocalVariables|SetDirection (Math|Vector2D|Normalize2D (- (Variables|/Game/01_BP/03_Character/TopDownCharacter.TopDownCharacter_C|Getgrid%20Index (Variables|Default|GetSpellOwner)) pos))))
  (LocalVariables|SetCurrentTarget (- (Variables|/Game/01_BP/03_Character/TopDownCharacter.TopDownCharacter_C|Getgrid%20Index (Variables|Default|GetSpellOwner)) _output_get))
  (for _index (range 0 (Variables|Default|Getm_Distances))
    (if (and (>= (.x (LocalVariables|GetCurrentTarget)) 0.0) (>= (.y (LocalVariables|GetCurrentTarget)) 0.0))
      (Utilities|Casting|CastToTopDownCharacter (.unitonthistile (.Value (Utilities|Map|Find (Variables|/Game/01_BP/Grid/GridBehaviours.GridBehaviours_C|Getstruct_Tiles (LocalVariables|GetGridManager)) (LocalVariables|GetCurrentTarget))))
        (:then
          _)
        (:CastFailed
          _))
      (Utilities|Array|AddUnique (LocalVariables|GetAffectedTiles) (.m_tiles_index (.Value (Utilities|Map|Find (Variables|/Game/01_BP/Grid/GridBehaviours.GridBehaviours_C|Getstruct_Tiles (LocalVariables|GetGridManager)) (LocalVariables|GetCurrentTarget)))))
      (LocalVariables|SetCurrentTarget (- (LocalVariables|GetCurrentTarget) (LocalVariables|GetDirection)))))
  (LocalVariables|SetCurrentPosition (- (Variables|/Game/01_BP/03_Character/TopDownCharacter.TopDownCharacter_C|Getgrid%20Index (Variables|Default|GetSpellOwner)) (* (LocalVariables|GetDirection) (Math|Conversions|ToFloat(Integer) (Variables|Default|Getm_Distances)))))
  (Utilities|Casting|CastToTopDownCharacter (.unitonthistile (.Value (Utilities|Map|Find (Variables|/Game/01_BP/Grid/GridBehaviours.GridBehaviours_C|Getstruct_Tiles (LocalVariables|GetGridManager)) (LocalVariables|GetCurrentPosition))))
    (:then
      (if (not (Utilities|Array|ContainsItem (LocalVariables|GetAffectedTiles) (LocalVariables|GetCurrentPosition)))
        (Utilities|Array|AddUnique (LocalVariables|GetAffectedTiles) (LocalVariables|GetCurrentPosition)))
      (while (.bSuccess (Utilities|Casting|CastToTopDownCharacter (.unitonthistile (.Value (Utilities|Map|Find (Variables|/Game/01_BP/Grid/GridBehaviours.GridBehaviours_C|Getstruct_Tiles (LocalVariables|GetGridManager)) (LocalVariables|GetCurrentPosition))))))
        (LocalVariables|SetCurrentPosition (- (LocalVariables|GetCurrentPosition) (LocalVariables|GetDirection)))
        (if (not (.bSuccess (Utilities|Casting|CastToTopDownCharacter (.unitonthistile (.Value (Utilities|Map|Find (Variables|/Game/01_BP/Grid/GridBehaviours.GridBehaviours_C|Getstruct_Tiles (LocalVariables|GetGridManager)) (LocalVariables|GetCurrentPosition)))))))
          (if (Math|Boolean|ANDBoolean (== (.unitonthistile (.Value (Utilities|Map|Find (Variables|/Game/01_BP/Grid/GridBehaviours.GridBehaviours_C|Getstruct_Tiles (LocalVariables|GetGridManager)) (LocalVariables|GetCurrentPosition)))) 0) (Utilities|Enum|NotEqual(Enum) (.m_typesoftile (.Value (Utilities|Map|Find (Variables|/Game/01_BP/Grid/GridBehaviours.GridBehaviours_C|Getstruct_Tiles (LocalVariables|GetGridManager)) (LocalVariables|GetCurrentPosition)))) "NewEnumerator6") (Utilities|Enum|NotEqual(Enum) (.m_typesoftile (.Value (Utilities|Map|Find (Variables|/Game/01_BP/Grid/GridBehaviours.GridBehaviours_C|Getstruct_Tiles (LocalVariables|GetGridManager)) (LocalVariables|GetCurrentPosition)))) "NewEnumerator5"))
            (Utilities|Array|AddUnique (LocalVariables|GetAffectedTiles) (LocalVariables|GetCurrentPosition))
            (return (LocalVariables|GetAffectedTiles))))))
    (:CastFailed
      (return (LocalVariables|GetAffectedTiles)))))