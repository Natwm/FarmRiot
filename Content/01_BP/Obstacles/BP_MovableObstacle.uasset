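; Movable grid obstacle that occupies a tile and can be pushed to another.
; Shortly after BeginPlay it scans every Grid tile for the one nearest its location, registers itself there and snaps to that tile's world location.
; E_GetPush clears its current tile, stores the new index and registers on that tile, without setting the actor's location in this graph.
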(event Custom|E_GetPush
  (params (NewPosition :type Vector%202D%20Structure))
  (CallFunction|RemoveUnitonThisTIles)
  (bind _output_get (Variables|Default|SetGrid%20Index NewPosition))
  (CallFunction|SetUnitonTile _output_get))

(event EventBeginPlay
  (|CallParentFunction)
  (Utilities|FlowControl|Delay 0.2)
  (CallFunction|SetGridIndexandSnapIt))

(event Collision|EventActorBeginOverlap
  (params (OtherActor :type Actor%20Object%20Reference))
  (|CallParentFunction OtherActor) ; This node is disabled and will not be called.\nDrag off pins to build functionality.
)

(event EventTick
  (params (DeltaSeconds :type Float%20%28single-precision%29))
  (|CallParentFunction DeltaSeconds) ; This node is disabled and will not be called.\nDrag off pins to build functionality.
)

(fn ConstructionScript
  (|CallParentFunction))

(fn SetGridIndexandSnapIt
  (bind _grid (Variables|Default|GetGrid))
  (bind _struct_tiles (Variables|/Game/01_BP/Grid/GridBehaviours.GridBehaviours_C|Getstruct_Tiles _grid))
  (bind _keys (Utilities|Map|Keys _struct_tiles))
  (for _array_element _keys
    (if (< (Math|Vector|VectorLength (- (.m_tiles_worldlocation (.Value (Utilities|Map|Find _struct_tiles _array_element))) (Transformation|GetActorLocation self))) (LocalVariables|GetClosesDistance))
      (LocalVariables|SetClosesDistance (Math|Vector|VectorLength (- (.m_tiles_worldlocation (.Value (Utilities|Map|Find _struct_tiles _array_element))) (Transformation|GetActorLocation self))))
      (LocalVariables|SetCloses%20Index (.m_tiles_index (.Value (Utilities|Map|Find _struct_tiles _array_element))))))
  (CallFunction|SetUnitonTile (LocalVariables|GetCloses%20Index))
  (Transformation|SetActorLocation (.m_tiles_worldlocation (.Value (Utilities|Map|Find (Variables|/Game/01_BP/Grid/GridBehaviours.GridBehaviours_C|Getstruct_Tiles _grid) (LocalVariables|GetCloses%20Index)))) false false))