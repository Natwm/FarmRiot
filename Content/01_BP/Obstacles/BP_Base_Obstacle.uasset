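; Base obstacle actor that registers itself as the occupant of a tile in the GridBehaviours map.
; BeginPlay waits briefly, then caches the grid; the snap call in the event graph is unwired.
; The snap function scans all tiles for the nearest, occupies it and moves the actor there.
; Occupying writes self, tile type, cost and a fruit flag from a BP_Obstacle_Fruit cast; removal clears only the occupant.
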(event EventBeginPlay
  (Utilities|FlowControl|Delay 0.2)
  (bind _returnvalue (Actor|GetActorOfClass "/Game/01_BP/Grid/GridBehaviours.GridBehaviours_C"))
  (Variables|Default|SetGrid _returnvalue))

(event Collision|EventActorBeginOverlap
  (params (OtherActor :type Actor%20Object%20Reference)))

(event EventTick
  (params (DeltaSeconds :type Float%20%28single-precision%29)))

(fn ConstructionScript)

(fn SetGridIndexandSnaptoLocation
  (bind _grid (Variables|Default|GetGrid))
  (bind _struct_tiles (Variables|/Game/01_BP/Grid/GridBehaviours.GridBehaviours_C|Getstruct_Tiles _grid))
  (bind _keys (Utilities|Map|Keys _struct_tiles))
  (for _array_element _keys
    (if (< (Math|Vector|VectorLength (- (.m_tiles_worldlocation (.Value (Utilities|Map|Find _struct_tiles _array_element))) (Transformation|GetActorLocation self))) (LocalVariables|GetClosesDistace))
      (LocalVariables|SetClosesDistace (Math|Vector|VectorLength (- (.m_tiles_worldlocation (.Value (Utilities|Map|Find _struct_tiles _array_element))) (Transformation|GetActorLocation self))))
      (LocalVariables|SetClosesIndex (.m_tiles_index (.Value (Utilities|Map|Find _struct_tiles _array_element))))))
  (CallFunction|SetUnitonTile (LocalVariables|GetClosesIndex))
  (Transformation|SetActorLocation (.m_tiles_worldlocation (.Value (Utilities|Map|Find (Variables|/Game/01_BP/Grid/GridBehaviours.GridBehaviours_C|Getstruct_Tiles _grid) (LocalVariables|GetClosesIndex)))) false false))

(fn SetUnitonTile
  (params (grid%20Index :type Vector%202D%20Structure))
  (bind _grid (Variables|Default|GetGrid))
  (bind _grid_2 (Variables|Default|GetGrid))
  (bind _struct_tiles (Variables|/Game/01_BP/Grid/GridBehaviours.GridBehaviours_C|Getstruct_Tiles _grid))
  (bind _struct_tiles_2 (Variables|/Game/01_BP/Grid/GridBehaviours.GridBehaviours_C|Getstruct_Tiles _grid_2))
  (Utilities|Map|Add _struct_tiles_2 (Variables|Default|Getgrid%20Index) (Utilities|Struct|MakeTiles_Struct (.tileactor (.Value (Utilities|Map|Find _struct_tiles_2 (Variables|Default|Getgrid%20Index)))) 0 (.tilecost (.Value (Utilities|Map|Find _struct_tiles_2 (Variables|Default|Getgrid%20Index)))) (.m_typesoftile (.Value (Utilities|Map|Find _struct_tiles_2 (Variables|Default|Getgrid%20Index)))) (.m_tiles_worldlocation (.Value (Utilities|Map|Find _struct_tiles_2 (Variables|Default|Getgrid%20Index)))) (.m_tiles_index (.Value (Utilities|Map|Find _struct_tiles_2 (Variables|Default|Getgrid%20Index)))) (.finalcost (.Value (Utilities|Map|Find _struct_tiles_2 (Variables|Default|Getgrid%20Index)))) (.costfromstart (.Value (Utilities|Map|Find _struct_tiles_2 (Variables|Default|Getgrid%20Index)))) (.estimatedcosttotarget (.Value (Utilities|Map|Find _struct_tiles_2 (Variables|Default|Getgrid%20Index)))) (.previoustiles (.Value (Utilities|Map|Find _struct_tiles_2 (Variables|Default|Getgrid%20Index)))) (.height (.Value (Utilities|Map|Find _struct_tiles_2 (Variables|Default|Getgrid%20Index)))) (.isfruit (.Value (Utilities|Map|Find _struct_tiles_2 (Variables|Default|Getgrid%20Index))))))
  (Variables|Default|Setgrid%20Index grid%20Index)
  (Utilities|Map|Add _struct_tiles (Variables|Default|Getgrid%20Index) (Utilities|Struct|MakeTiles_Struct (.tileactor (.Value (Utilities|Map|Find _struct_tiles (Variables|Default|Getgrid%20Index)))) self (Default|GetTilesCost _grid (Variables|Default|GetTileType)) (Variables|Default|GetTileType) (.m_tiles_worldlocation (.Value (Utilities|Map|Find _struct_tiles (Variables|Default|Getgrid%20Index)))) (.m_tiles_index (.Value (Utilities|Map|Find _struct_tiles (Variables|Default|Getgrid%20Index)))) (.finalcost (.Value (Utilities|Map|Find _struct_tiles (Variables|Default|Getgrid%20Index)))) (.costfromstart (.Value (Utilities|Map|Find _struct_tiles (Variables|Default|Getgrid%20Index)))) (.estimatedcosttotarget (.Value (Utilities|Map|Find _struct_tiles (Variables|Default|Getgrid%20Index)))) (.previoustiles (.Value (Utilities|Map|Find _struct_tiles (Variables|Default|Getgrid%20Index)))) (.height (.Value (Utilities|Map|Find _struct_tiles (Variables|Default|Getgrid%20Index)))) (.AsBP%20Obstacle%20Fruit (Utilities|Casting|CastToBP_Obstacle_Fruit self)))))

(fn RemoveUnitonThisTIles
  (bind _grid (Variables|Default|GetGrid))
  (bind _grid_index (Variables|Default|GetGrid%20Index))
  (bind _struct_tiles (Variables|/Game/01_BP/Grid/GridBehaviours.GridBehaviours_C|Getstruct_Tiles _grid))
  (bind _value (Utilities|Map|Find _struct_tiles _grid_index))
  (Utilities|Map|Add _struct_tiles (Variables|Default|GetGrid%20Index) (Utilities|Struct|MakeTiles_Struct (.tileactor _value) 0 (.tilecost _value) (.m_typesoftile _value) (.m_tiles_worldlocation _value) (.m_tiles_index _value) (.finalcost _value) (.costfromstart _value) (.estimatedcosttotarget _value) (.previoustiles _value) (.height _value) (.isfruit _value))))