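; A camera pawn Blueprint that rotates from player yaw and pitch axis input.
; Yaw input rotates the actor in world space and pitch input rotates it locally, both scaled by a rotation speed, which keeps yaw free of tilt.
; Each tick clamps the pitch between minimum and maximum limits by resetting the rotation with the current yaw.
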(event EventTick
  (params (DeltaSeconds :type Float%20%28single-precision%29))
  (bind _returnvalue (Transformation|GetActorRotation))
  (bind _minyrotation (Variables|Default|GetMinYRotation))
  (bind _maxyrotation (Variables|Default|GetMaxYrotation))
  (bind _returnvalue_2 (< (.pitch _returnvalue) _minyrotation))
  (if (or _returnvalue_2 (> (.pitch _returnvalue) _maxyrotation))
    (Transformation|SetActorRotation (Math|Rotator|MakeRotator 0.0 (Math|Float|SelectFloat _minyrotation _maxyrotation _returnvalue_2) (.yaw _returnvalue)))))

(event Input|AxisEvents|InputAxisCameraRotationYaw
  (params (AxisValue :type Float%20%28single-precision%29))
  (Class|Actor|AddActorWorldRotation (Math|Rotator|MakeRotator 0.0 0.0 (* AxisValue (Variables|Default|GetRotationSpeed)))))

(event Input|AxisEvents|InputAxisCameraRotationPitch
  (params (AxisValue :type Float%20%28single-precision%29))
  (Transformation|AddActorLocalRotation (Math|Rotator|MakeRotator 0.0 (* AxisValue (Variables|Default|GetRotationSpeed)) 0.0) false false))

(fn ConstructionScript)