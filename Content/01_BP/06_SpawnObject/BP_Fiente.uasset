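; BP_Fiente is a destructible grid hazard that highlights its surrounding tiles as egg zones and explodes on moving characters nearby.
; On spawn it caches neighbouring tiles from the Grid, and its tile check triggers the explosion for any moving TopDownCharacter found there.
; The explosion damages that character, clears the highlight and tile occupancy, then destroys the actor after a short delay.
; Losing all life also triggers the explosion, without a target.
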(event Custom|E_Explosion
  (params (Character :type Top%20Down%20Character%20Object%20Reference))
  (Utilities|IsValid Character
    (:Is%20Valid
      (Default|ETakeDamage Character (Variables|Default|GetDamage) Character))
    (:Is%20Not%20Valid
      _))
  (Default|HighlightEggsZones (Variables|Default|GetGrid) (Variables|Default|GetTilesPositionArround) false)
  (CallFunction|RemoveUnitonThisTIles)
  (Utilities|FlowControl|Delay 0.2)
  (Actor|DestroyActor))

(event Custom|E_CheckNearTiles
  (for _array_element (Variables|Default|GetTilesPositionArround)
    (bind _astop_down_character (Utilities|Casting|CastToTopDownCharacter (.unitonthistile (.Value (Utilities|Map|Find (Variables|/Game/01_BP/Grid/GridBehaviours.GridBehaviours_C|Getstruct_Tiles (Variables|Default|GetGrid)) _array_element)))))
    (if (Variables|/Game/01_BP/03_Character/TopDownCharacter.TopDownCharacter_C|GetIsMoving _astop_down_character)
      (CallFunction|EExplosion _astop_down_character))))

(event Custom|E_ShowTiles
  (bind _targatableindexes (Default|GetArround (Variables|Default|GetGrid) (Variables|Default|Getgrid%20Index)))
  (bind _output_get (Variables|Default|SetTilesPositionArround _targatableindexes))
  (Default|HighlightEggsZones (Variables|Default|GetGrid) _output_get false))

(event Custom|E_TakeDamage
  (params (AmountOfDamage :type Integer))
  (bind _output_get (Variables|Default|SetLife (- (Variables|Default|GetLife) AmountOfDamage)))
  (if (<= _output_get 0)
    (CallFunction|EExplosion)))

(event EventBeginPlay
  (|CallParentFunction)
  (Utilities|FlowControl|Delay 0.2)
  (bind _targatableindexes (Default|GetArround (Variables|Default|GetGrid) (Variables|Default|Getgrid%20Index)))
  (bind _output_get (Variables|Default|SetTilesPositionArround _targatableindexes))
  (Default|HighlightEggsZones (Variables|Default|GetGrid) _output_get true))

(event Collision|EventActorBeginOverlap
  (params (OtherActor :type Actor%20Object%20Reference))
  (|CallParentFunction OtherActor) ; This node is disabled and will not be called.\nDrag off pins to build functionality.
)

(event EventTick
  (params (DeltaSeconds :type Float%20%28single-precision%29))
  (|CallParentFunction DeltaSeconds) ; This node is disabled and will not be called.\nDrag off pins to build functionality.
)

(fn ConstructionScript
  (|CallParentFunction))