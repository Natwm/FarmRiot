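; BP_Eggs is a control spell that drops a BP_Fiente (poop) actor on a targeted grid tile.
; On use, it spawns the actor at the tile's world location, unless a TopDownCharacter stands there or the tile is one of two excluded types.
; SetUnitOnATile then rewrites the tile's struct to register the dropping as its unit, and passes it the grid index, spell damage and caster's owner.
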(event EventEUseSpellonTarget
  (params (Grid :type Grid%20Behaviours%20Object%20Reference) (Target%20position :type Vector%202D%20Structure) (SpellOwner :type Top%20Down%20Character%20Object%20Reference))
  (bind _struct_tiles (Variables|/Game/01_BP/Grid/GridBehaviours.GridBehaviours_C|Getstruct_Tiles Grid))
  (bind _value (Utilities|Map|Find _struct_tiles Target%20position))
  (if (Math|Boolean|ANDBoolean (not (.bSuccess (Utilities|Casting|CastToTopDownCharacter (.unitonthistile _value)))) (Utilities|Enum|NotEqual(Enum) (.m_typesoftile _value) "NewEnumerator5") (Utilities|Enum|NotEqual(Enum) (.m_typesoftile _value) "NewEnumerator6"))
    (bind _returnvalue (Game|SpawnActorfromClass "/Game/01_BP/06_SpawnObject/BP_Fiente.BP_Fiente_C" (Math|Transform|MakeTransform (.m_tiles_worldlocation _value) "0, 0, 0" "1,1,1") "Undefined" 0 0))
    (CallFunction|SetUnitonATile Grid Target%20position _returnvalue)))

(fn ConstructionScript
  (|CallParentFunction))

(fn SetUnitonATile
  (params (Grid :type Grid%20Behaviours%20Object%20Reference) (target :type Vector%202D%20Structure) (Fiente :type BP%20Fiente%20Object%20Reference))
  (LocalVariables|SetGridManager Grid)
  (LocalVariables|SetTargetVector2 target)
  (LocalVariables|SetFienteBP Fiente)
  (Utilities|Map|Add (Variables|/Game/01_BP/Grid/GridBehaviours.GridBehaviours_C|Getstruct_Tiles (LocalVariables|GetGridManager)) (LocalVariables|GetTargetVector2) (Utilities|Struct|MakeTiles_Struct (.tileactor (.Value (Utilities|Map|Find (Variables|/Game/01_BP/Grid/GridBehaviours.GridBehaviours_C|Getstruct_Tiles (LocalVariables|GetGridManager)) (LocalVariables|GetTargetVector2)))) 0 (.tilecost (.Value (Utilities|Map|Find (Variables|/Game/01_BP/Grid/GridBehaviours.GridBehaviours_C|Getstruct_Tiles (LocalVariables|GetGridManager)) (LocalVariables|GetTargetVector2)))) (.m_typesoftile (.Value (Utilities|Map|Find (Variables|/Game/01_BP/Grid/GridBehaviours.GridBehaviours_C|Getstruct_Tiles (LocalVariables|GetGridManager)) (LocalVariables|GetTargetVector2)))) (.m_tiles_worldlocation (.Value (Utilities|Map|Find (Variables|/Game/01_BP/Grid/GridBehaviours.GridBehaviours_C|Getstruct_Tiles (LocalVariables|GetGridManager)) (LocalVariables|GetTargetVector2)))) (.m_tiles_index (.Value (Utilities|Map|Find (Variables|/Game/01_BP/Grid/GridBehaviours.GridBehaviours_C|Getstruct_Tiles (LocalVariables|GetGridManager)) (LocalVariables|GetTargetVector2)))) (.finalcost (.Value (Utilities|Map|Find (Variables|/Game/01_BP/Grid/GridBehaviours.GridBehaviours_C|Getstruct_Tiles (LocalVariables|GetGridManager)) (LocalVariables|GetTargetVector2)))) (.costfromstart (.Value (Utilities|Map|Find (Variables|/Game/01_BP/Grid/GridBehaviours.GridBehaviours_C|Getstruct_Tiles (LocalVariables|GetGridManager)) (LocalVariables|GetTargetVector2)))) (.estimatedcosttotarget (.Value (Utilities|Map|Find (Variables|/Game/01_BP/Grid/GridBehaviours.GridBehaviours_C|Getstruct_Tiles (LocalVariables|GetGridManager)) (LocalVariables|GetTargetVector2)))) (.previoustiles (.Value (Utilities|Map|Find (Variables|/Game/01_BP/Grid/GridBehaviours.GridBehaviours_C|Getstruct_Tiles (LocalVariables|GetGridManager)) (LocalVariables|GetTargetVector2)))) (.height (.Value (Utilities|Map|Find (Variables|/Game/01_BP/Grid/GridBehaviours.GridBehaviours_C|Getstruct_Tiles (LocalVariables|GetGridManager)) (LocalVariables|GetTargetVector2)))) (.isfruit (.Value (Utilities|Map|Find (Variables|/Game/01_BP/Grid/GridBehaviours.GridBehaviours_C|Getstruct_Tiles (LocalVariables|GetGridManager)) (LocalVariables|GetTargetVector2))))))
  (Variables|/Game/01_BP/Obstacles/BP_Base_Obstacle.BP_Base_Obstacle_C|SetGrid%20Index (LocalVariables|GetFienteBP) (LocalVariables|GetTargetVector2))
  (Utilities|Map|Add (Variables|/Game/01_BP/Grid/GridBehaviours.GridBehaviours_C|Getstruct_Tiles (LocalVariables|GetGridManager)) (LocalVariables|GetTargetVector2) (Utilities|Struct|MakeTiles_Struct (.tileactor (.Value (Utilities|Map|Find (Variables|/Game/01_BP/Grid/GridBehaviours.GridBehaviours_C|Getstruct_Tiles (LocalVariables|GetGridManager)) (LocalVariables|GetTargetVector2)))) (LocalVariables|GetFienteBP) (.tilecost (.Value (Utilities|Map|Find (Variables|/Game/01_BP/Grid/GridBehaviours.GridBehaviours_C|Getstruct_Tiles (LocalVariables|GetGridManager)) (LocalVariables|GetTargetVector2)))) (.m_typesoftile (.Value (Utilities|Map|Find (Variables|/Game/01_BP/Grid/GridBehaviours.GridBehaviours_C|Getstruct_Tiles (LocalVariables|GetGridManager)) (LocalVariables|GetTargetVector2)))) (.m_tiles_worldlocation (.Value (Utilities|Map|Find (Variables|/Game/01_BP/Grid/GridBehaviours.GridBehaviours_C|Getstruct_Tiles (LocalVariables|GetGridManager)) (LocalVariables|GetTargetVector2)))) (.m_tiles_index (.Value (Utilities|Map|Find (Variables|/Game/01_BP/Grid/GridBehaviours.GridBehaviours_C|Getstruct_Tiles (LocalVariables|GetGridManager)) (LocalVariables|GetTargetVector2)))) (.finalcost (.Value (Utilities|Map|Find (Variables|/Game/01_BP/Grid/GridBehaviours.GridBehaviours_C|Getstruct_Tiles (LocalVariables|GetGridManager)) (LocalVariables|GetTargetVector2)))) (.costfromstart (.Value (Utilities|Map|Find (Variables|/Game/01_BP/Grid/GridBehaviours.GridBehaviours_C|Getstruct_Tiles (LocalVariables|GetGridManager)) (LocalVariables|GetTargetVector2)))) (.estimatedcosttotarget (.Value (Utilities|Map|Find (Variables|/Game/01_BP/Grid/GridBehaviours.GridBehaviours_C|Getstruct_Tiles (LocalVariables|GetGridManager)) (LocalVariables|GetTargetVector2)))) (.previoustiles (.Value (Utilities|Map|Find (Variables|/Game/01_BP/Grid/GridBehaviours.GridBehaviours_C|Getstruct_Tiles (LocalVariables|GetGridManager)) (LocalVariables|GetTargetVector2)))) (.height (.Value (Utilities|Map|Find (Variables|/Game/01_BP/Grid/GridBehaviours.GridBehaviours_C|Getstruct_Tiles (LocalVariables|GetGridManager)) (LocalVariables|GetTargetVector2)))) (.isfruit (.Value (Utilities|Map|Find (Variables|/Game/01_BP/Grid/GridBehaviours.GridBehaviours_C|Getstruct_Tiles (LocalVariables|GetGridManager)) (LocalVariables|GetTargetVector2))))))
  (Variables|/Game/01_BP/06_SpawnObject/BP_Fiente.BP_Fiente_C|SetDamage (LocalVariables|GetFienteBP) (Variables|Default|Getm_Degats))
  (Variables|/Game/01_BP/06_SpawnObject/BP_Fiente.BP_Fiente_C|SetPoopOwner (LocalVariables|GetFienteBP) (Variables|/Game/01_BP/03_Character/TopDownCharacter.TopDownCharacter_C|Getm_PawnOwner (Variables|Default|GetSpellOwner))))