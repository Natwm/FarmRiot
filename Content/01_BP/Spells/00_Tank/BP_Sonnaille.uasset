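; Tank spell Blueprint, Sonnaille, that links same-owner units in its target area to the casting Tank.
; Targeting takes attackable tiles from the origin, passes them through the grid's tiles-around query and highlights them, with range raised by one at player height 2.
; On use, it stores the Tank in each allied unit's TankIntoSonnaille, undoes the height bonus, deselects the spell and plays FMOD audio.
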(event EventEShowTilesTargetedbySpell
  (params (Origin%20Index :type Vector%202D%20Structure) (Grid :type Grid%20Behaviours%20Object%20Reference) (Show%20Tiles :type Boolean))
  (if (== (Variables|/Game/01_BP/03_Character/TopDownCharacter.TopDownCharacter_C|GetPlayerHeight (Variables|Default|GetSpellOwner)) 2)
    (Math|Integer|IncrementInt (Variables|Default|Getm_Distances)
      (:%20%20
        _)))
  (if (> (Utilities|Array|Length (Variables|Default|GetReachableTarger)) 0)
    (Default|HighlightAttackableTiles Grid (Variables|Default|GetReachableTarger) false)
    (Utilities|Array|Clear (Variables|Default|GetReachableTarger)))
  (bind _newlocalvar_01 (CallFunction|GetAttackableTiles Origin%20Index Grid))
  (bind _output_get (Variables|Default|SetReachableTarger _newlocalvar_01))
  (bind _tilesarroundtheplayer (Default|GetTileArround Grid _output_get (Variables|/Game/01_BP/03_Character/TopDownCharacter.TopDownCharacter_C|Getgrid%20Index (Variables|Default|GetSpellOwner))))
  (bind _output_get_2 (Variables|Default|SetReachableTarger _tilesarroundtheplayer))
  (Default|HighlightAttackableTiles Grid _output_get_2 Show%20Tiles))

(event EventEUseSpellonTarget
  (params (Grid :type Grid%20Behaviours%20Object%20Reference) (Target%20position :type Vector%202D%20Structure) (SpellOwner :type Top%20Down%20Character%20Object%20Reference))
  (for _array_element (Variables|Default|GetReachableTarger)
    (bind _astop_down_character (Utilities|Casting|CastToTopDownCharacter (.unitonthistile (.Value (Utilities|Map|Find (Variables|/Game/01_BP/Grid/GridBehaviours.GridBehaviours_C|Getstruct_Tiles Grid) _array_element)))))
    (if (Utilities|Enum|Equal(Enum) (Variables|/Game/01_BP/03_Character/TopDownCharacter.TopDownCharacter_C|Getm_PawnOwner _astop_down_character) (Variables|/Game/01_BP/03_Character/TopDownCharacter.TopDownCharacter_C|Getm_PawnOwner SpellOwner))
      (bind _astank_character (Utilities|Casting|CastToTank_Character SpellOwner))
      (Variables|/Game/01_BP/03_Character/TopDownCharacter.TopDownCharacter_C|SetTankIntoSonnaille _astop_down_character _astank_character)))
  (if (== (Variables|/Game/01_BP/03_Character/TopDownCharacter.TopDownCharacter_C|GetPlayerHeight (Variables|Default|GetSpellOwner)) 2)
    (Math|Integer|DecrementInt (Variables|Default|Getm_Distances)
      (:%20%20
        _)))
  (Default|EDeselectSpeel SpellOwner)
  (Class|FMODAudioComponent|Play (Variables|Default|GetAttaque_FMODAudio)))

(fn ConstructionScript
  (|CallParentFunction))