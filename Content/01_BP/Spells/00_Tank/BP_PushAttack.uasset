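; Tank push spell for grid combat that damages an enemy in reach, or targets a movable obstacle, and shoves it away using GetDirection.
; EUseSpellonTarget validates the tile and unit, runs PushActionResult or PushObjectResult, then calls ReduceInit and deselects the spell.
; A free destination tile receives the pushed unit or object, while a blocking character takes half damage.
; An enemy pushed into an obstacle receives a debuff instead of moving.
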(event EventEUseSpellonTarget
  (params (Grid :type Grid%20Behaviours%20Object%20Reference) (Target%20position :type Vector%202D%20Structure) (SpellOwner :type Top%20Down%20Character%20Object%20Reference))
  (bind _struct_tiles (Variables|/Game/01_BP/Grid/GridBehaviours.GridBehaviours_C|Getstruct_Tiles Grid))
  (bind _value (Utilities|Map|Find _struct_tiles Target%20position))
  (bind (_asbp_movable_obstacle _bsuccess) (Utilities|Casting|CastToBP_MovableObstacle (.unitonthistile _value)))
  (if (Utilities|Array|ContainsItem (Variables|Default|GetReachableTarger) Target%20position)
    (bind _astop_down_character (Utilities|Casting|CastToTopDownCharacter (.unitonthistile _value))
      (:then
        (if (Math|Boolean|ANDBoolean (stale _bsuccess) (Utilities|Enum|NotEqual(Enum) (.m_typesoftile _value) "NewEnumerator5") (Utilities|Enum|NotEqual(Enum) (.m_typesoftile _value) "NewEnumerator6") (Utilities|Enum|NotEqual(Enum) (Variables|/Game/01_BP/03_Character/TopDownCharacter.TopDownCharacter_C|Getm_PawnOwner _astop_down_character) (Variables|/Game/01_BP/03_Character/TopDownCharacter.TopDownCharacter_C|Getm_PawnOwner SpellOwner)))
          (Default|ETakeDamage _astop_down_character (Variables|Default|Getm_Degats))
          (CallFunction|PushActionResult _astop_down_character SpellOwner Grid)
          (CallFunction|ReduceInit :!label _label)
          (Default|EDeselectSpeel SpellOwner)
          (else
            (if _bsuccess :!label _label_2
              (CallFunction|PushObjectResult Grid _asbp_movable_obstacle)
              (goto _label)))))
      (:CastFailed
        (goto _label_2)))))

(fn ConstructionScript
  (|CallParentFunction))

(fn PushActionResult
  (params (SpeelTarget :type Top%20Down%20Character%20Object%20Reference) (SpeelCaster :type Top%20Down%20Character%20Object%20Reference) (GridManager :type Grid%20Behaviours%20Object%20Reference))
  (LocalVariables|SetTarget SpeelTarget)
  (LocalVariables|SetCaster SpeelCaster)
  (LocalVariables|SetGrid GridManager)
  (if (== (.unitonthistile (.Value (Utilities|Map|Find (Variables|/Game/01_BP/Grid/GridBehaviours.GridBehaviours_C|Getstruct_Tiles (LocalVariables|GetGrid)) (CallFunction|GetDirection (Variables|/Game/01_BP/03_Character/TopDownCharacter.TopDownCharacter_C|Getgrid%20Index (LocalVariables|GetTarget)) (Variables|/Game/01_BP/03_Character/TopDownCharacter.TopDownCharacter_C|Getgrid%20Index (LocalVariables|GetCaster)))))) 0)
    (Transformation|SetActorLocation (LocalVariables|GetTarget) (.m_tiles_worldlocation (.Value (Utilities|Map|Find (Variables|/Game/01_BP/Grid/GridBehaviours.GridBehaviours_C|Getstruct_Tiles (LocalVariables|GetGrid)) (CallFunction|GetDirection (Variables|/Game/01_BP/03_Character/TopDownCharacter.TopDownCharacter_C|Getgrid%20Index (LocalVariables|GetTarget)) (Variables|/Game/01_BP/03_Character/TopDownCharacter.TopDownCharacter_C|Getgrid%20Index (LocalVariables|GetCaster)))))) false false)
    (Variables|/Game/01_BP/03_Character/TopDownCharacter.TopDownCharacter_C|Setgrid%20Index (LocalVariables|GetTarget) (.m_tiles_index (.Value (Utilities|Map|Find (Variables|/Game/01_BP/Grid/GridBehaviours.GridBehaviours_C|Getstruct_Tiles (LocalVariables|GetGrid)) (CallFunction|GetDirection (Variables|/Game/01_BP/03_Character/TopDownCharacter.TopDownCharacter_C|Getgrid%20Index (LocalVariables|GetTarget)) (Variables|/Game/01_BP/03_Character/TopDownCharacter.TopDownCharacter_C|Getgrid%20Index (LocalVariables|GetCaster)))))))
    (elif (.bSuccess (Utilities|Casting|CastToTopDownCharacter (.unitonthistile (.Value (Utilities|Map|Find (Variables|/Game/01_BP/Grid/GridBehaviours.GridBehaviours_C|Getstruct_Tiles (LocalVariables|GetGrid)) (CallFunction|GetDirection (Variables|/Game/01_BP/03_Character/TopDownCharacter.TopDownCharacter_C|Getgrid%20Index (LocalVariables|GetTarget)) (Variables|/Game/01_BP/03_Character/TopDownCharacter.TopDownCharacter_C|Getgrid%20Index (LocalVariables|GetCaster))))))))
      (Default|ETakeDamage (.AsTop%20Down%20Character (Utilities|Casting|CastToTopDownCharacter (.unitonthistile (.Value (Utilities|Map|Find (Variables|/Game/01_BP/Grid/GridBehaviours.GridBehaviours_C|Getstruct_Tiles (LocalVariables|GetGrid)) (CallFunction|GetDirection (Variables|/Game/01_BP/03_Character/TopDownCharacter.TopDownCharacter_C|Getgrid%20Index (LocalVariables|GetTarget)) (Variables|/Game/01_BP/03_Character/TopDownCharacter.TopDownCharacter_C|Getgrid%20Index (LocalVariables|GetCaster)))))))) (/ (Variables|Default|Getm_Degats) 2))
      (else
        ;[1 1 1] Apply a debuf on the speed
        (if (.bSuccess (Utilities|Casting|CastToBP_Base_Obstacle (.unitonthistile (.Value (Utilities|Map|Find (Variables|/Game/01_BP/Grid/GridBehaviours.GridBehaviours_C|Getstruct_Tiles (LocalVariables|GetGrid)) (CallFunction|GetDirection (Variables|/Game/01_BP/03_Character/TopDownCharacter.TopDownCharacter_C|Getgrid%20Index (LocalVariables|GetTarget)) (Variables|/Game/01_BP/03_Character/TopDownCharacter.TopDownCharacter_C|Getgrid%20Index (LocalVariables|GetCaster))))))))
          (Default|EApplyDebuff (LocalVariables|GetTarget) 1))))))

(fn PushObjectResult
  (params (GridManager :type Grid%20Behaviours%20Object%20Reference) (Obstacle :type BP%20Movable%20Obstacle%20Object%20Reference))
  (LocalVariables|SetGrid GridManager)
  (bind _output_get (LocalVariables|SetObstacleToPush Obstacle))
  (if (== (.unitonthistile (.Value (Utilities|Map|Find (Variables|/Game/01_BP/Grid/GridBehaviours.GridBehaviours_C|Getstruct_Tiles (LocalVariables|GetGrid)) (CallFunction|GetDirection (Variables|/Game/01_BP/Obstacles/BP_Base_Obstacle.BP_Base_Obstacle_C|GetGrid%20Index _output_get) (Variables|/Game/01_BP/03_Character/TopDownCharacter.TopDownCharacter_C|Getgrid%20Index (Variables|Default|GetSpellOwner)))))) 0)
    (Transformation|SetActorLocation (LocalVariables|GetObstacleToPush) (.m_tiles_worldlocation (.Value (Utilities|Map|Find (Variables|/Game/01_BP/Grid/GridBehaviours.GridBehaviours_C|Getstruct_Tiles (LocalVariables|GetGrid)) (CallFunction|GetDirection (Variables|/Game/01_BP/Obstacles/BP_Base_Obstacle.BP_Base_Obstacle_C|GetGrid%20Index _output_get) (Variables|/Game/01_BP/03_Character/TopDownCharacter.TopDownCharacter_C|Getgrid%20Index (Variables|Default|GetSpellOwner)))))) false false)
    (Default|SetUnitonTile (LocalVariables|GetObstacleToPush) (.m_tiles_index (.Value (Utilities|Map|Find (Variables|/Game/01_BP/Grid/GridBehaviours.GridBehaviours_C|Getstruct_Tiles (LocalVariables|GetGrid)) (CallFunction|GetDirection (Variables|/Game/01_BP/Obstacles/BP_Base_Obstacle.BP_Base_Obstacle_C|GetGrid%20Index _output_get) (Variables|/Game/01_BP/03_Character/TopDownCharacter.TopDownCharacter_C|Getgrid%20Index (Variables|Default|GetSpellOwner)))))))
    (elif (.bSuccess (Utilities|Casting|CastToTopDownCharacter (.unitonthistile (.Value (Utilities|Map|Find (Variables|/Game/01_BP/Grid/GridBehaviours.GridBehaviours_C|Getstruct_Tiles (LocalVariables|GetGrid)) (CallFunction|GetDirection (Variables|/Game/01_BP/Obstacles/BP_Base_Obstacle.BP_Base_Obstacle_C|GetGrid%20Index _output_get) (Variables|/Game/01_BP/03_Character/TopDownCharacter.TopDownCharacter_C|Getgrid%20Index (Variables|Default|GetSpellOwner))))))))
      (Default|ETakeDamage (.AsTop%20Down%20Character (Utilities|Casting|CastToTopDownCharacter (.unitonthistile (.Value (Utilities|Map|Find (Variables|/Game/01_BP/Grid/GridBehaviours.GridBehaviours_C|Getstruct_Tiles (LocalVariables|GetGrid)) (CallFunction|GetDirection (Variables|/Game/01_BP/Obstacles/BP_Base_Obstacle.BP_Base_Obstacle_C|GetGrid%20Index _output_get) (Variables|/Game/01_BP/03_Character/TopDownCharacter.TopDownCharacter_C|Getgrid%20Index (Variables|Default|GetSpellOwner)))))))) (/ (Variables|Default|Getm_Degats) 2)))))