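; Basic spell for a grid-based tactics game that highlights its targetable tiles and damages an enemy character on the chosen tile.
; Targeting scans tiles within a min/max Manhattan range, with an optional height check, and caches them for clearing highlights.
; Casting rejects same-owner units and two tile types, then deducts initiative cost and deselects the spell.
; Pathfinding, straight-line, minimum-distance and direction helpers are defined but not called here.
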(event Custom|E_UseSpellOnTarget
  (params (Grid :type Grid%20Behaviours%20Object%20Reference) (Target%20position :type Vector%202D%20Structure) (SpellOwner :type Top%20Down%20Character%20Object%20Reference))
  (bind _struct_tiles (Variables|/Game/01_BP/Grid/GridBehaviours.GridBehaviours_C|Getstruct_Tiles Grid))
  (bind _value (Utilities|Map|Find _struct_tiles Target%20position))
  (bind (_astop_down_character _bsuccess) (Utilities|Casting|CastToTopDownCharacter (.unitonthistile _value)))
  (if (Math|Boolean|ANDBoolean _bsuccess (Utilities|Enum|NotEqual(Enum) (.m_typesoftile _value) "NewEnumerator5") (Utilities|Enum|NotEqual(Enum) (.m_typesoftile _value) "NewEnumerator6") (Utilities|Enum|NotEqual(Enum) (Variables|/Game/01_BP/03_Character/TopDownCharacter.TopDownCharacter_C|Getm_PawnOwner _astop_down_character) (Variables|/Game/01_BP/03_Character/TopDownCharacter.TopDownCharacter_C|Getm_PawnOwner SpellOwner)))
    (Default|ETakeDamage _astop_down_character (Variables|Value|Getm_Degats))
    (CallFunction|ReduceInit)
    (Default|EDeselectSpeel SpellOwner)))

(event Custom|E_ShowTilesTargetedBySpell
  (params (Origin%20Index :type Vector%202D%20Structure) (Grid :type Grid%20Behaviours%20Object%20Reference) (Show%20Tiles :type Boolean))
  (if (> (Utilities|Array|Length (Variables|Default|GetReachableTarger)) 0)
    (Default|HighlightAttackableTiles Grid (Variables|Default|GetReachableTarger) false)
    (Utilities|Array|Clear (Variables|Default|GetReachableTarger)))
  (bind _newlocalvar_01 (CallFunction|GetAttackableTiles Origin%20Index Grid))
  (bind _output_get (Variables|Default|SetReachableTarger _newlocalvar_01))
  (Default|HighlightAttackableTiles Grid _output_get Show%20Tiles))

(fn ConstructionScript)

(fn GetReachableTarget
  (params (Origin%20Index :type Vector%202D%20Structure) (Distance :type Integer) (Grid :type Grid%20Behaviours%20Object%20Reference))
  (LocalVariables|SetFirstIndex Origin%20Index)
  (LocalVariables|Setm_Distance Distance)
  (bind _keys (Utilities|Map|Keys (Variables|/Game/01_BP/Grid/GridBehaviours.GridBehaviours_C|Getstruct_Tiles Grid)))
  (bind _array_element (Utilities|Array|ForEachLoopwithBreak _keys :!label _label)
    (:LoopBody
      (bind _output_get (LocalVariables|SetTargetIndex _array_element))
      (if (Math|Boolean|ORBoolean (!= (.unitonthistile (.Value (Utilities|Map|Find (Variables|/Game/01_BP/Grid/GridBehaviours.GridBehaviours_C|Getstruct_Tiles Grid) _output_get))) 0) (Utilities|Enum|Equal(Enum) (.m_typesoftile (.Value (Utilities|Map|Find (Variables|/Game/01_BP/Grid/GridBehaviours.GridBehaviours_C|Getstruct_Tiles Grid) _output_get))) "NewEnumerator6") (Utilities|Enum|Equal(Enum) (.m_typesoftile (.Value (Utilities|Map|Find (Variables|/Game/01_BP/Grid/GridBehaviours.GridBehaviours_C|Getstruct_Tiles Grid) _output_get))) "NewEnumerator5") (> (Default|GetEstimatedCosttoTarget Grid (LocalVariables|GetFirstIndex) (LocalVariables|GetTargetIndex)) (LocalVariables|Getm_Distance)))
        (goto _label Break)))
    (:Completed
      (bind _reachable_tiles (Default|FindPathtoTarget Grid (LocalVariables|GetFirstIndex) (LocalVariables|GetTargetIndex) (LocalVariables|Getm_Distance) true (Variables|flag|Getm_PassThroughWalls) true))
      (return _reachable_tiles))))

(fn GetAttackableTiles
  (params (NewParam :type Vector%202D%20Structure) (grid :type Grid%20Behaviours%20Object%20Reference))
  (bind _m_distances (Variables|Value|Getm_Distances))
  (bind _m_distances_2 (Variables|Value|Getm_Distances))
  (for _index (range (* _m_distances_2 -1) _m_distances_2)
    (for _index_2 (range (* _m_distances -1) _m_distances)
      (if (.ReturnValue (CallFunction|DoesThisTilesIsCorrect NewParam _index _index_2 grid))
        (Utilities|Array|AddUnique (LocalVariables|GetNewLocalVar_0) (.ValidPosition (CallFunction|DoesThisTilesIsCorrect NewParam _index _index_2 grid))))))
  (return (LocalVariables|GetNewLocalVar_0)))

(fn ReduceInit
  (Variables|/Game/01_BP/03_Character/TopDownCharacter.TopDownCharacter_C|Setm_Initiative (Variables|Default|GetSpellOwner) (- (Variables|/Game/01_BP/03_Character/TopDownCharacter.TopDownCharacter_C|Getm_Initiative (Variables|Default|GetSpellOwner)) (Variables|Value|Getm_Cost))))

(fn GetDirection
  (params (Target :type Vector%202D%20Structure) (Caster :type Vector%202D%20Structure))
  (return (+ Target (- Target Caster))))

(fn GetReachableTargetatMinimumDistances
  (params (Targets :type Array%20of%20Vector%202D%20Structures) (unitPos :type Vector%202D%20Structure))
  (for _array_element Targets
    (if (> (Math|Float|Round (Class|KismetMathLibrary|DistanceSquared2D _array_element unitPos)) (Variables|Value|GetMinDistance))
      (Utilities|Array|AddUnique (LocalVariables|GetTiles) _array_element)))
  (return (LocalVariables|GetTiles)))

(fn DoesThisTilesIsCorrect
  (params (InVec :type Vector%202D%20Structure) (X :type Integer) (Y :type Integer) (grid :type Grid%20Behaviours%20Object%20Reference))
  (bind _returnvalue (Math|Conversions|ToFloat(Integer) X))
  (bind _returnvalue_2 (Math|Conversions|ToFloat(Integer) Y))
  (bind (_x _y) (Math|Vector2D|BreakVector2D InVec))
  (bind _struct_tiles (Variables|/Game/01_BP/Grid/GridBehaviours.GridBehaviours_C|Getstruct_Tiles grid))
  (bind _isaffectbyheight (Variables|flag|GetIsAffectByHeight))
  (bind _mindistance (Variables|Value|GetMinDistance))
  (bind _m_distances (Variables|Value|Getm_Distances))
  (bind _returnvalue_3 (Math|Vector2D|MakeVector2D _returnvalue _returnvalue_2))
  (bind _returnvalue_4 (not _isaffectbyheight))
  (bind _returnvalue_5 (Math|Conversions|ToFloat(Integer) _mindistance))
  (bind _returnvalue_6 (Math|Conversions|ToFloat(Integer) _m_distances))
  (bind _returnvalue_7 (+ InVec _returnvalue_3))
  (bind _value (Utilities|Map|Find _struct_tiles _returnvalue_7))
  (bind (_x_2 _y_2) (Math|Vector2D|BreakVector2D _returnvalue_7))
  (bind _returnvalue_8 (!= (.unitonthistile _value) 0))
  (bind _can_walk_on_this_tile_valid (Default|CanJumponThisTiles grid (.height _value)))
  (bind _returnvalue_9 (- _x_2 _x))
  (bind _returnvalue_10 (- _y_2 _y))
  (bind _bsuccess (Utilities|Casting|CastToTopDownCharacter (.unitonthistile _value)))
  (bind _returnvalue_11 (Utilities|Enum|Equal(Enum) (.m_typesoftile _value) "NewEnumerator5"))
  (bind _returnvalue_12 (Utilities|Enum|Equal(Enum) (.m_typesoftile _value) "NewEnumerator6"))
  (bind _returnvalue_13 (not _bsuccess))
  (bind _returnvalue_14 (Math|Float|Absolute(Float) _returnvalue_9))
  (bind _returnvalue_15 (Math|Float|Absolute(Float) _returnvalue_10))
  (bind _returnvalue_16 (or _can_walk_on_this_tile_valid _returnvalue_4))
  (bind _returnvalue_17 (Math|Boolean|ORBoolean _returnvalue_8 _returnvalue_12 _returnvalue_11 _returnvalue_13))
  (bind _returnvalue_18 (+ _returnvalue_14 _returnvalue_15))
  (bind _returnvalue_19 (> _returnvalue_18 _returnvalue_5))
  (bind _returnvalue_20 (<= _returnvalue_18 _returnvalue_6))
  (bind _returnvalue_21 (and _returnvalue_16 _returnvalue_17))
  (bind _returnvalue_22 (and _returnvalue_19 _returnvalue_20))
  (bind _returnvalue_23 (and _returnvalue_22 _returnvalue_21))
  (if _returnvalue_23
    (return _returnvalue_23 _returnvalue_7)))

(fn CheckForward
  (params (Array :type Array%20of%20Vector%202D%20Structures))
  (bind _spellowner (Variables|Default|GetSpellOwner))
  (bind _grid_index (Variables|/Game/01_BP/03_Character/TopDownCharacter.TopDownCharacter_C|Getgrid%20Index _spellowner))
  (bind (_x _y) (Math|Vector2D|BreakVector2D _grid_index))
  (for _array_element Array
    (if (or (== (.X (Math|Vector2D|BreakVector2D _array_element)) _x) (== (.Y (Math|Vector2D|BreakVector2D _array_element)) _y))
      (Utilities|Array|AddUnique (LocalVariables|GetReachableTaget) _array_element)))
  (return (LocalVariables|GetReachableTaget)))