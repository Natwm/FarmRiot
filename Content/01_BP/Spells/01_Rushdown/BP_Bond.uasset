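; Rushdown leap spell for the grid tactics game that teleports the caster to a reachable, unoccupied tile of an allowed type.
; Dropping one height level pushes neighboring characters away from the landing tile; dropping two also damages them first.
; Push resolves height differences and collisions into damage, or a debuff when an obstacle blocks the target.
; The spell then updates caster height and tile, calls ReduceInit and deselects.
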(event EventEUseSpellonTarget
  (params (Grid :type Grid%20Behaviours%20Object%20Reference) (Target%20position :type Vector%202D%20Structure) (SpellOwner :type Top%20Down%20Character%20Object%20Reference))
  (bind _struct_tiles (Variables|/Game/01_BP/Grid/GridBehaviours.GridBehaviours_C|Getstruct_Tiles Grid))
  (bind _value (Utilities|Map|Find _struct_tiles Target%20position))
  (if (Utilities|Array|ContainsItem (Variables|Default|GetReachableTarger) Target%20position)
    (if (Math|Boolean|ANDBoolean (not (.bSuccess (Utilities|Casting|CastToTopDownCharacter (.unitonthistile _value)))) (Utilities|Enum|NotEqual(Enum) (.m_typesoftile _value) "NewEnumerator5") (Utilities|Enum|NotEqual(Enum) (.m_typesoftile _value) "NewEnumerator6"))
      (switch int (- (Variables|/Game/01_BP/03_Character/TopDownCharacter.TopDownCharacter_C|GetPlayerHeight (Variables|Default|GetSpellOwner)) (.height _value))
        (:Default
          _)
        (:0
          _)
        (:1
          (Variables|Default|SetUseSpecial false)
          (CallFunction|SpecialJumpAction Grid Target%20position :!label _label))
        (:2
          (Variables|Default|SetUseSpecial true)
          (goto _label)))
      (Transformation|SetActorLocation (Variables|Default|GetSpellOwner) (.m_tiles_worldlocation _value) false false)
      (Variables|/Game/01_BP/03_Character/TopDownCharacter.TopDownCharacter_C|SetPlayerHeight (Variables|Default|GetSpellOwner) (.height _value))
      (Default|GetUnitonTile (Variables|Default|GetSpellOwner) Target%20position)
      (CallFunction|ReduceInit)
      (Default|EDeselectSpeel (Variables|Default|GetSpellOwner)))))

(fn ConstructionScript
  (|CallParentFunction))

(fn GetTilesArroundforEffects
  (params (Grid :type Grid%20Behaviours%20Object%20Reference) (TargetIndex :type Vector%202D%20Structure))
  (LocalVariables|SetGridManager Grid)
  (bind _targatableindexes (Default|GetArround Grid TargetIndex))
  (for _array_element _targatableindexes
    (if (!= (.unitonthistile (.Value (Utilities|Map|Find (Variables|/Game/01_BP/Grid/GridBehaviours.GridBehaviours_C|Getstruct_Tiles (LocalVariables|GetGridManager)) _array_element))) 0)
      (Utilities|Casting|CastToTopDownCharacter (.unitonthistile (.Value (Utilities|Map|Find (Variables|/Game/01_BP/Grid/GridBehaviours.GridBehaviours_C|Getstruct_Tiles (LocalVariables|GetGridManager)) _array_element)))
        (:then
          _)
        (:CastFailed
          (Utilities|Casting|CastToBP_MovableObstacle (.unitonthistile (.Value (Utilities|Map|Find (Variables|/Game/01_BP/Grid/GridBehaviours.GridBehaviours_C|Getstruct_Tiles (LocalVariables|GetGridManager)) _array_element))))))
      (Utilities|Array|AddUnique (LocalVariables|GetTargetableUnit) _array_element)))
  (return (LocalVariables|GetTargetableUnit)))

(fn DamageUnitbyPropultion
  (params (Tagets :type Array%20of%20Vector%202D%20Structures) (Grid%20Manager :type Grid%20Behaviours%20Object%20Reference))
  (LocalVariables|SetGridManager Grid%20Manager)
  (for _array_element Tagets
    (if (Math|Vector|NotEqual(Vector) _array_element (Variables|/Game/01_BP/03_Character/TopDownCharacter.TopDownCharacter_C|Getgrid%20Index (Variables|Default|GetSpellOwner)) 0.0001)
      (bind _astop_down_character (Utilities|Casting|CastToTopDownCharacter (.unitonthistile (.Value (Utilities|Map|Find (Variables|/Game/01_BP/Grid/GridBehaviours.GridBehaviours_C|Getstruct_Tiles (LocalVariables|GetGridManager)) _array_element)))))
      (if (!= _astop_down_character (Variables|Default|GetSpellOwner))
        (Default|ETakeDamage _astop_down_character (Variables|Default|GetmaxDegats))))))

(fn PushbyJump
  (params (GridManager :type Grid%20Behaviours%20Object%20Reference) (Targets :type Array%20of%20Vector%202D%20Structures) (JumpPosition :type Vector%202D%20Structure))
  (LocalVariables|SetGrid GridManager)
  (for _array_element Targets
    (bind _astop_down_character (Utilities|Casting|CastToTopDownCharacter (.unitonthistile (.Value (Utilities|Map|Find (Variables|/Game/01_BP/Grid/GridBehaviours.GridBehaviours_C|Getstruct_Tiles (LocalVariables|GetGrid)) _array_element)))))
    (CallFunction|Push _astop_down_character JumpPosition (LocalVariables|GetGrid))))

(fn Push
  (params (SpellTargetPosition :type Top%20Down%20Character%20Object%20Reference) (FuturSpellOwnerPosition :type Vector%202D%20Structure) (GridManager :type Grid%20Behaviours%20Object%20Reference))
  (LocalVariables|SetTarget SpellTargetPosition)
  (LocalVariables|SetCaster FuturSpellOwnerPosition)
  (LocalVariables|SetGrid GridManager)
  (if (== (.unitonthistile (.Value (Utilities|Map|Find (Variables|/Game/01_BP/Grid/GridBehaviours.GridBehaviours_C|Getstruct_Tiles (LocalVariables|GetGrid)) (CallFunction|GetDirection (Variables|/Game/01_BP/03_Character/TopDownCharacter.TopDownCharacter_C|Getgrid%20Index (LocalVariables|GetTarget)) (LocalVariables|GetCaster))))) 0)
    (if (>= (- (Variables|/Game/01_BP/03_Character/TopDownCharacter.TopDownCharacter_C|GetPlayerHeight (LocalVariables|GetTarget)) (.height (.Value (Utilities|Map|Find (Variables|/Game/01_BP/Grid/GridBehaviours.GridBehaviours_C|Getstruct_Tiles (LocalVariables|GetGrid)) (CallFunction|GetDirection (Variables|/Game/01_BP/03_Character/TopDownCharacter.TopDownCharacter_C|Getgrid%20Index (LocalVariables|GetTarget)) (LocalVariables|GetCaster)))))) 0)
      (switch int (- (Variables|/Game/01_BP/03_Character/TopDownCharacter.TopDownCharacter_C|GetPlayerHeight (LocalVariables|GetTarget)) (.height (.Value (Utilities|Map|Find (Variables|/Game/01_BP/Grid/GridBehaviours.GridBehaviours_C|Getstruct_Tiles (LocalVariables|GetGrid)) (CallFunction|GetDirection (Variables|/Game/01_BP/03_Character/TopDownCharacter.TopDownCharacter_C|Getgrid%20Index (LocalVariables|GetTarget)) (LocalVariables|GetCaster))))))
        (:0
          _)
        (:1
          (Default|ETakeDamage (LocalVariables|GetTarget) (/ (Variables|Default|GetmaxDegats) 2)))
        (:2
          (Default|ETakeDamage (LocalVariables|GetTarget) (Variables|Default|GetmaxDegats))))
      (Transformation|SetActorLocation (LocalVariables|GetTarget) (.m_tiles_worldlocation (.Value (Utilities|Map|Find (Variables|/Game/01_BP/Grid/GridBehaviours.GridBehaviours_C|Getstruct_Tiles (LocalVariables|GetGrid)) (CallFunction|GetDirection (Variables|/Game/01_BP/03_Character/TopDownCharacter.TopDownCharacter_C|Getgrid%20Index (LocalVariables|GetTarget)) (LocalVariables|GetCaster))))) false false)
      (Default|GetUnitonTile (LocalVariables|GetTarget))
      (Default|ETakeDamage (LocalVariables|GetTarget) (Variables|Default|GetmaxDegats))
      (else
        (Default|ETakeDamage (LocalVariables|GetTarget) (/ (Variables|Default|GetmaxDegats) 2))))
    (elif (.bSuccess (Utilities|Casting|CastToTopDownCharacter (.unitonthistile (.Value (Utilities|Map|Find (Variables|/Game/01_BP/Grid/GridBehaviours.GridBehaviours_C|Getstruct_Tiles (LocalVariables|GetGrid)) (CallFunction|GetDirection (Variables|/Game/01_BP/03_Character/TopDownCharacter.TopDownCharacter_C|Getgrid%20Index (LocalVariables|GetTarget)) (LocalVariables|GetCaster)))))))
      (Default|ETakeDamage (.AsTop%20Down%20Character (Utilities|Casting|CastToTopDownCharacter (.unitonthistile (.Value (Utilities|Map|Find (Variables|/Game/01_BP/Grid/GridBehaviours.GridBehaviours_C|Getstruct_Tiles (LocalVariables|GetGrid)) (CallFunction|GetDirection (Variables|/Game/01_BP/03_Character/TopDownCharacter.TopDownCharacter_C|Getgrid%20Index (LocalVariables|GetTarget)) (LocalVariables|GetCaster))))))) (/ (Variables|Default|GetmaxDegats) 2))
      (else
        ;[1 1 1] Apply a debuf on the speed
        (if (.bSuccess (Utilities|Casting|CastToBP_Base_Obstacle (.unitonthistile (.Value (Utilities|Map|Find (Variables|/Game/01_BP/Grid/GridBehaviours.GridBehaviours_C|Getstruct_Tiles (LocalVariables|GetGrid)) (CallFunction|GetDirection (Variables|/Game/01_BP/03_Character/TopDownCharacter.TopDownCharacter_C|Getgrid%20Index (LocalVariables|GetTarget)) (LocalVariables|GetCaster)))))))
          (Default|EApplyDebuff (LocalVariables|GetTarget) 1))))))

(fn SpecialJumpAction
  (params (grid :type Grid%20Behaviours%20Object%20Reference) (targetIndex :type Vector%202D%20Structure))
  (LocalVariables|Setmanager grid)
  (if (Variables|Default|GetUseSpecial)
    (CallFunction|DamageUnitbyPropultion (CallFunction|GetTilesArroundforEffects (LocalVariables|Getmanager) targetIndex) (LocalVariables|Getmanager)))
  (CallFunction|PushbyJump (LocalVariables|Getmanager) (CallFunction|GetTilesArroundforEffects (LocalVariables|Getmanager) targetIndex) targetIndex))