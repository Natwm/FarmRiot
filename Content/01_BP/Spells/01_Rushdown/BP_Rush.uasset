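; Rush spell for a grid tactics game: the caster charges in a line, damaging characters on the way.
; Targeting highlights reachable tiles, optionally straight-line only, raising range when PlayerHeight is 2; the matching decrement never runs.
; On use, NewFunction0 collects tiles along the direction, extending past occupied tiles toward a free valid one.
; Characters there take MaxDegats, then the caster teleports to the last tile; RushActionResult serves only disconnected logic.
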(event EventEUseSpellonTarget
  (params (Grid :type Grid%20Behaviours%20Object%20Reference) (Target%20position :type Vector%202D%20Structure) (SpellOwner :type Top%20Down%20Character%20Object%20Reference))
  (bind _affectedtile (CallFunction|NewFunction0 Grid Target%20position SpellOwner))
  (for _array_element _affectedtile
    (bind _astop_down_character (Utilities|Casting|CastToTopDownCharacter (.unitonthistile (.Value (Utilities|Map|Find (Variables|/Game/01_BP/Grid/GridBehaviours.GridBehaviours_C|Getstruct_Tiles Grid) _array_element))))
      (:then
        (Default|ETakeDamage _astop_down_character (Variables|Default|GetmaxDegats)))
      (:CastFailed
        _))
    (if (< (CallFunction|ManhattanDistance (Variables|Default|Gettest_0_0) _array_element) 0.0)
      (Variables|Default|Settest_0_0 (.m_tiles_index (.Value (Utilities|Map|Find (Variables|/Game/01_BP/Grid/GridBehaviours.GridBehaviours_C|Getstruct_Tiles Grid) _array_element))))))
  (Variables|Default|Settest_0_0 (Utilities|Array|Get(acopy) _affectedtile (Utilities|Array|LastIndex _affectedtile)))
  (Transformation|SetActorLocation (Variables|Default|GetSpellOwner) (.m_tiles_worldlocation (.Value (Utilities|Map|Find (Variables|/Game/01_BP/Grid/GridBehaviours.GridBehaviours_C|Getstruct_Tiles Grid) (Variables|Default|Gettest_0_0)))) false false)
  (Default|GetUnitonTile (Variables|Default|GetSpellOwner) (.m_tiles_index (.Value (Utilities|Map|Find (Variables|/Game/01_BP/Grid/GridBehaviours.GridBehaviours_C|Getstruct_Tiles Grid) (Variables|Default|Gettest_0_0)))))
  (Default|EDeselectSpeel (Variables|Default|GetSpellOwner))
  (Class|FMODAudioComponent|Play (Variables|Default|GetAttaque_FMODAudio)))

(event EventEShowTilesTargetedbySpell
  (params (Origin%20Index :type Vector%202D%20Structure) (Grid :type Grid%20Behaviours%20Object%20Reference) (Show%20Tiles :type Boolean))
  (if (== (Variables|/Game/01_BP/03_Character/TopDownCharacter.TopDownCharacter_C|GetPlayerHeight (Variables|Default|GetSpellOwner)) 2)
    (Math|Integer|IncrementInt (Variables|Default|Getm_Distances)
      (:%20%20
        (Math|Integer|IncrementInt (Variables|Default|GetMinDistance)
          (:%20%20
            _)))))
  (if (> (Utilities|Array|Length (Variables|Default|GetReachableTarger)) 0)
    (Default|HighlightAttackableTiles Grid (Variables|Default|GetReachableTarger) false)
    (Utilities|Array|Clear (Variables|Default|GetReachableTarger)))
  (bind _newlocalvar_01 (CallFunction|GetAttackableTiles Origin%20Index Grid))
  (bind _reachablestargets (CallFunction|GetReachableTargetatMinimumDistances _newlocalvar_01 Origin%20Index))
  (if (Variables|Flag|GetIsStraightLineq)
    (bind _reachabletiles (CallFunction|CheckForward _reachablestargets))
    (bind _output_get (Variables|Default|SetReachableTarger _reachabletiles))
    (Default|HighlightAttackableTiles Grid _output_get Show%20Tiles)))

(fn ConstructionScript
  (|CallParentFunction))

(fn RushActionResult
  (params (Grid :type Grid%20Behaviours%20Object%20Reference) (target :type Vector%202D%20Structure))
  (LocalVariables|SetLocatTargetTile target)
  (LocalVariables|SetDirection (Math|Vector2D|Normalize2D (- (Variables|/Game/01_BP/03_Character/TopDownCharacter.TopDownCharacter_C|Getgrid%20Index (Variables|Default|GetSpellOwner)) target)))
  (for _index (range (Variables|Default|Getm_Distances) (Variables|Default|Getm_Distances))
    (LocalVariables|SetLocatTargetTile (- (Variables|/Game/01_BP/03_Character/TopDownCharacter.TopDownCharacter_C|Getgrid%20Index (Variables|Default|GetSpellOwner)) (LocalVariables|GetDirection)))
    (if (.bSuccess (Utilities|Casting|CastToTopDownCharacter (.unitonthistile (.Value (Utilities|Map|Find (Variables|/Game/01_BP/Grid/GridBehaviours.GridBehaviours_C|Getstruct_Tiles Grid) (LocalVariables|GetLocatTargetTile))))))
      (Utilities|Array|AddUnique (LocalVariables|GetAffectedTiles) (LocalVariables|GetLocatTargetTile))))
  (while (.bSuccess (Utilities|Casting|CastToTopDownCharacter (.unitonthistile (.Value (Utilities|Map|Find (Variables|/Game/01_BP/Grid/GridBehaviours.GridBehaviours_C|Getstruct_Tiles Grid) (LocalVariables|GetLocatTargetTile))))))
    (Utilities|Array|AddUnique (LocalVariables|GetAffectedTiles) (LocalVariables|GetLocatTargetTile))
    (LocalVariables|SetLocatTargetTile (- (LocalVariables|GetLocatTargetTile) (LocalVariables|GetDirection)))
    (if (not (.bSuccess (Utilities|Casting|CastToTopDownCharacter (.unitonthistile (.Value (Utilities|Map|Find (Variables|/Game/01_BP/Grid/GridBehaviours.GridBehaviours_C|Getstruct_Tiles Grid) (LocalVariables|GetLocatTargetTile)))))))
      (if (Math|Boolean|ANDBoolean (== (.unitonthistile (.Value (Utilities|Map|Find (Variables|/Game/01_BP/Grid/GridBehaviours.GridBehaviours_C|Getstruct_Tiles Grid) (LocalVariables|GetLocatTargetTile)))) 0) (Utilities|Enum|NotEqual(Enum) (.m_typesoftile (.Value (Utilities|Map|Find (Variables|/Game/01_BP/Grid/GridBehaviours.GridBehaviours_C|Getstruct_Tiles Grid) (LocalVariables|GetLocatTargetTile)))) "NewEnumerator6") (Utilities|Enum|NotEqual(Enum) (.m_typesoftile (.Value (Utilities|Map|Find (Variables|/Game/01_BP/Grid/GridBehaviours.GridBehaviours_C|Getstruct_Tiles Grid) (LocalVariables|GetLocatTargetTile)))) "NewEnumerator5"))
        (Utilities|Array|AddUnique (LocalVariables|GetAffectedTiles) (LocalVariables|GetLocatTargetTile))
        (return (LocalVariables|GetAffectedTiles))))))

(fn RushActionApply
  (params (Grid :type Grid%20Behaviours%20Object%20Reference) (target :type Vector%202D%20Structure))
  (bind _struct_tiles (Variables|/Game/01_BP/Grid/GridBehaviours.GridBehaviours_C|Getstruct_Tiles Grid))
  (bind _value (Utilities|Map|Find _struct_tiles target))
  (bind (_astop_down_character _bsuccess) (Utilities|Casting|CastToTopDownCharacter (.unitonthistile _value)))
  (if _bsuccess
    (Default|ETakeDamage _astop_down_character (Variables|Default|GetmaxDegats))))

(fn NewFunction0
  (params (grid :type Grid%20Behaviours%20Object%20Reference%20%28by%20ref%29) (pos :type Vector%202D%20Structure) (target :type Top%20Down%20Character%20Object%20Reference))
  (LocalVariables|SetGridManager grid)
  (bind _output_get (LocalVariables|SetDirection (Math|Vector2D|Normalize2D (- (Variables|/Game/01_BP/03_Character/TopDownCharacter.TopDownCharacter_C|Getgrid%20Index (Variables|Default|GetSpellOwner)) pos))))
  (LocalVariables|SetCurrentTarget (- (Variables|/Game/01_BP/03_Character/TopDownCharacter.TopDownCharacter_C|Getgrid%20Index (Variables|Default|GetSpellOwner)) _output_get))
  (for _index (range 0 (Variables|Default|Getm_Distances))
    (Utilities|Casting|CastToTopDownCharacter (.unitonthistile (.Value (Utilities|Map|Find (Variables|/Game/01_BP/Grid/GridBehaviours.GridBehaviours_C|Getstruct_Tiles (LocalVariables|GetGridManager)) (LocalVariables|GetCurrentTarget))))
      (:then
        _)
      (:CastFailed
        _))
    (Utilities|Array|AddUnique (LocalVariables|GetAffectedTiles) (.m_tiles_index (.Value (Utilities|Map|Find (Variables|/Game/01_BP/Grid/GridBehaviours.GridBehaviours_C|Getstruct_Tiles (LocalVariables|GetGridManager)) (LocalVariables|GetCurrentTarget)))))
    (LocalVariables|SetCurrentTarget (- (LocalVariables|GetCurrentTarget) (LocalVariables|GetDirection))))
  (LocalVariables|SetCurrentPosition (- (Variables|/Game/01_BP/03_Character/TopDownCharacter.TopDownCharacter_C|Getgrid%20Index (Variables|Default|GetSpellOwner)) (* (LocalVariables|GetDirection) (Math|Conversions|ToFloat(Integer) (Variables|Default|Getm_Distances)))))
  (Utilities|Casting|CastToTopDownCharacter (.unitonthistile (.Value (Utilities|Map|Find (Variables|/Game/01_BP/Grid/GridBehaviours.GridBehaviours_C|Getstruct_Tiles (LocalVariables|GetGridManager)) (LocalVariables|GetCurrentPosition))))
    (:then
      (if (not (Utilities|Array|ContainsItem (LocalVariables|GetAffectedTiles) (LocalVariables|GetCurrentPosition)))
        (Utilities|Array|AddUnique (LocalVariables|GetAffectedTiles) (LocalVariables|GetCurrentPosition)))
      (while (.bSuccess (Utilities|Casting|CastToTopDownCharacter (.unitonthistile (.Value (Utilities|Map|Find (Variables|/Game/01_BP/Grid/GridBehaviours.GridBehaviours_C|Getstruct_Tiles (LocalVariables|GetGridManager)) (LocalVariables|GetCurrentPosition))))))
        (LocalVariables|SetCurrentPosition (- (LocalVariables|GetCurrentPosition) (LocalVariables|GetDirection)))
        (if (not (.bSuccess (Utilities|Casting|CastToTopDownCharacter (.unitonthistile (.Value (Utilities|Map|Find (Variables|/Game/01_BP/Grid/GridBehaviours.GridBehaviours_C|Getstruct_Tiles (LocalVariables|GetGridManager)) (LocalVariables|GetCurrentPosition)))))))
          (if (Math|Boolean|ANDBoolean (== (.unitonthistile (.Value (Utilities|Map|Find (Variables|/Game/01_BP/Grid/GridBehaviours.GridBehaviours_C|Getstruct_Tiles (LocalVariables|GetGridManager)) (LocalVariables|GetCurrentPosition)))) 0) (Utilities|Enum|NotEqual(Enum) (.m_typesoftile (.Value (Utilities|Map|Find (Variables|/Game/01_BP/Grid/GridBehaviours.GridBehaviours_C|Getstruct_Tiles (LocalVariables|GetGridManager)) (LocalVariables|GetCurrentPosition)))) "NewEnumerator6") (Utilities|Enum|NotEqual(Enum) (.m_typesoftile (.Value (Utilities|Map|Find (Variables|/Game/01_BP/Grid/GridBehaviours.GridBehaviours_C|Getstruct_Tiles (LocalVariables|GetGridManager)) (LocalVariables|GetCurrentPosition)))) "NewEnumerator5"))
            (Utilities|Array|AddUnique (LocalVariables|GetAffectedTiles) (LocalVariables|GetCurrentPosition))
            (return (LocalVariables|GetAffectedTiles))))))
    (:CastFailed
      (return (LocalVariables|GetAffectedTiles)))))