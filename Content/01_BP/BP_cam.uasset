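; BP_cam is a camera actor, judging by its name, that rotates from two input values with a limited pitch range.
; Event A applies yaw in world space and event B applies pitch in local space, both scaled by RotationSpeed.
; Tick snaps out-of-range pitch back to MinYRotation or MaxYrotation, keeping the current yaw.
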(event Custom|B
  (params (val :type Float%20%28single-precision%29))
  (Transformation|AddActorLocalRotation (Math|Rotator|MakeRotator 0.0 (* val (Variables|Default|GetRotation%20Speed)) 0.0) false false))

(event Custom|A
  (params (val :type Float%20%28single-precision%29))
  (Class|Actor|AddActorWorldRotation (Math|Rotator|MakeRotator 0.0 0.0 (* val (Variables|Default|GetRotation%20Speed)))))

(event EventTick
  (params (DeltaSeconds :type Float%20%28single-precision%29))
  (bind _returnvalue (Transformation|GetActorRotation))
  (bind _min_yrotation (Variables|Default|GetMin%20YRotation))
  (bind _max_yrotation (Variables|Default|GetMax%20Yrotation))
  (bind _returnvalue_2 (< (.pitch _returnvalue) _min_yrotation))
  (if (or _returnvalue_2 (> (.pitch _returnvalue) _max_yrotation))
    (Transformation|SetActorRotation (Math|Rotator|MakeRotator 0.0 (Math|Float|SelectFloat _min_yrotation _max_yrotation _returnvalue_2) (.yaw _returnvalue)))))

(fn ConstructionScript)