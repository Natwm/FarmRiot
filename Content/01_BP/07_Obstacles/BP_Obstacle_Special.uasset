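; BP_Obstacle_Special is an obstacle tile that applies a bonus or malus to the player it affects.
; On BeginPlay it snaps itself to a fixed height, keeping its X and Y position.
; E_SpecialEffect validates the player, then uses IsImpactSpeed to choose between changing speed and changing spell cost.
; TileType sets the modifier's sign, and cost changes are sent to every actor in the player's spell list.
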(event Custom|E_SpecialEffect
  (params (AffectedPlayer :type Top%20Down%20Character%20Object%20Reference))
  (Utilities|IsValid AffectedPlayer
    (:Is%20Valid
      (switch Utilities|FlowControl|Switch|SwitchonSpecial_Effect (Variables|Default|GetIsImpactSpeed)
        (:NewEnumerator0
          (CallFunction|AffectPlayerSpeed AffectedPlayer))
        (:NewEnumerator1
          (CallFunction|AffectPlayerSpellCost AffectedPlayer))))))

(event EventBeginPlay
  (bind _returnvalue (Transformation|GetActorLocation))
  (|CallParentFunction)
  (Transformation|SetActorLocation (Math|Vector|MakeVector (.x _returnvalue) (.y _returnvalue) -104.0) false false))

(event Collision|EventActorBeginOverlap
  (params (OtherActor :type Actor%20Object%20Reference))
  (|CallParentFunction OtherActor) ; This node is disabled and will not be called.\nDrag off pins to build functionality.
)

(event EventTick
  (params (DeltaSeconds :type Float%20%28single-precision%29))
  (|CallParentFunction DeltaSeconds) ; This node is disabled and will not be called.\nDrag off pins to build functionality.
)

(fn ConstructionScript
  (|CallParentFunction))

(fn AffectPlayerSpeed
  (params (Player :type Top%20Down%20Character%20Object%20Reference))
  (bind _speedmodifier (Variables|Modifier|GetSpeedModifier))
  (switch Utilities|FlowControl|Switch|SwitchonTileProfiles (Variables|Default|GetTileType)
    (:NewEnumerator7
      (Variables|/Game/01_BP/03_Character/TopDownCharacter.TopDownCharacter_C|SetCurrenteSpeed Player (+ (Variables|/Game/01_BP/03_Character/TopDownCharacter.TopDownCharacter_C|GetCurrenteSpeed Player) _speedmodifier)))
    (:NewEnumerator8
      (Variables|/Game/01_BP/03_Character/TopDownCharacter.TopDownCharacter_C|SetCurrenteSpeed Player (- (Variables|/Game/01_BP/03_Character/TopDownCharacter.TopDownCharacter_C|GetCurrenteSpeed Player) _speedmodifier)))))

(fn AffectPlayerSpellCost
  (params (player :type Top%20Down%20Character%20Object%20Reference))
  (switch Utilities|FlowControl|Switch|SwitchonTileProfiles (Variables|Default|GetTileType)
    (:NewEnumerator7
      (LocalVariables|SetNewSpellModifer (* (Variables|Modifier|GetSpellCostModifier) -1)))
    (:NewEnumerator8
      (LocalVariables|SetNewSpellModifer (Variables|Modifier|GetSpellCostModifier))))
  (for _array_element (Variables|/Game/01_BP/03_Character/TopDownCharacter.TopDownCharacter_C|Getm_ListOfSpellActor player)
    (Default|EModifySpellCost _array_element (LocalVariables|GetNewSpellModifer))))